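; Player controller for a party-based game that routes camera, movement and action input to the currently possessed playable character.
; Number inputs swap to a party member from the game mode's list, skipping the current or knocked-out one, then possess it, refresh its UI and cached pawn reference.
; Cycling is delegated to the game mode.
; Debug keys test damage on nearby enemies or self, and party save/load.
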(event `self.ReceiveBeginPlay`
  (`self.ResetControlledPawn`))

(event `InputAxis|WalkForward`
  (params (AxisValue :type "Float (single-precision)"))
  ;[0 0 0] Character movement
  (`/Game/Blueprints/Characters/PlayableCharacters/PlayableCharacterBP.MoveForward` (cast `/Game/Blueprints/Characters/PlayableCharacters/PlayableCharacterBP` (`self.ControlledCharacter`) :!pure true) AxisValue))

(event `InputAxis|CameraLookRight`
  (params (AxisValue :type "Float (single-precision)"))
  ;[0 0 0] Camera controls
  (`Pawn.AddControllerYawInput` (`self.ControlledCharacter`) AxisValue))

(event `InputAxis|WalkRight`
  (params (AxisValue :type "Float (single-precision)"))
  ;[0 0 0] Character movement
  (`/Game/Blueprints/Characters/PlayableCharacters/PlayableCharacterBP.MoveRight` (cast `/Game/Blueprints/Characters/PlayableCharacters/PlayableCharacterBP` (`self.ControlledCharacter`) :!pure true) AxisValue))

(event `InputAxis|CameraLookUp`
  (params (AxisValue :type "Float (single-precision)"))
  ;[0 0 0] Camera controls
  (`Pawn.AddControllerPitchInput` (`self.ControlledCharacter`) AxisValue))

(event `InputAction|Action1`
  (params (Key :type "Key Structure"))
  ;[0 0 0] Actions
  (:`Pressed`
    (`/Game/Blueprints/Characters/BaseCharacterBP.Action1` (cast `/Game/Blueprints/Characters/PlayableCharacters/PlayableCharacterBP` (`self.ControlledCharacter`) :!pure true))))

(event `InputAction|SwapToCharacter1`
  (params (Key :type "Key Structure"))
  ;[0 0 0] Swap Characters (Character is chosen based on input)
  (:`Pressed`
    (`self.SwapCharacters` 0)))

(event `InputAction|CycleCharacter`
  (params (Key :type "Key Structure"))
  (bind _gamemoderef (`self.GameModeRef`))
  ;[0 0 0] Cycle Characters (Iteration)
  (:`Pressed`
    (`/Engine/EditorBlueprintResources/StandardMacros.IsValid` _gamemoderef
      (:`Is Valid`
        (`/Game/Blueprints/MainGameModeBP.Cycle Character` _gamemoderef self)))))

(event `InputAction|SwapToCharacter2`
  (params (Key :type "Key Structure"))
  ;[0 0 0] Swap Characters (Character is chosen based on input)
  (:`Pressed`
    (`self.SwapCharacters` 1)))

(event `InputAction|Action2`
  (params (Key :type "Key Structure"))
  ;[0 0 0] Actions
  (:`Pressed`
    (`/Game/Blueprints/Characters/BaseCharacterBP.Action2` (cast `/Game/Blueprints/Characters/PlayableCharacters/PlayableCharacterBP` (`self.ControlledCharacter`) :!pure true))))

(event `InputAction|SwapToCharacter3`
  (params (Key :type "Key Structure"))
  ;[0 0 0] Swap Characters (Character is chosen based on input)
  (:`Pressed`
    (`self.SwapCharacters` 2)))

(event `InputAction|DEBUG_KEY1`
  (params (Key :type "Key Structure"))
  (bind _controlledcharacter (`self.ControlledCharacter`))
  (bind _returnvalue (`self.K2_GetActorLocation` _controlledcharacter))
  ;[0.4667 0.2667 0] DEBUG (Num Pad 1): Checks nearby collision for nearby characters and does damage to them
  ; Tests ApplyDamage and ReceiveHealthChange custom events
  (:`Pressed`
    (bind _outhits (`KismetSystemLibrary.CapsuleTraceMulti` _returnvalue _returnvalue 70.0 70.0 "TraceTypeQuery1" false (`|MakeArray` _controlledcharacter :!type "Actor Object Reference") "ForDuration" true (struct :`R` 1.0 :`A` 1.0) (struct :`G` 1.0 :`A` 1.0) 2.0))
    (for _array_element _outhits
      (if (`self.ActorHasTag` (`.HitActor` (`GameplayStatics.BreakHitResult` _array_element)) "Enemy")
        (bind _asenemy_bp (cast `/Game/Blueprints/Characters/Enemy/EnemyBP` (`.HitActor` (`GameplayStatics.BreakHitResult` _array_element)) :!pure true))
        (`/Game/Blueprints/Characters/BaseCharacterBP.ApplyDamage` (cast `/Game/Blueprints/Characters/BaseCharacterBP` (`self.ControlledCharacter`) :!pure true) _asenemy_bp 10)
        (`KismetSystemLibrary.PrintString` (`KismetStringLibrary.Conv_IntToString` (`/Game/Blueprints/Characters/BaseCharacterBP.Health` _asenemy_bp)))
        (else
          (`KismetSystemLibrary.PrintString` "Didn't hit an enemy, but hit something!"))))))

(event `InputAction|DEBUG_KEY2`
  (params (Key :type "Key Structure"))
  (bind _asbase_character_bp (cast `/Game/Blueprints/Characters/BaseCharacterBP` (`self.ControlledCharacter`) :!pure true))
  ;[1 0.6118 0] DEBUG (Num Pad 2): Applies damage to self
  (:`Pressed`
    (`/Game/Blueprints/Characters/BaseCharacterBP.ApplyDamage` _asbase_character_bp _asbase_character_bp 50)
    (`KismetSystemLibrary.LogString` (`KismetStringLibrary.Conv_IntToString` (`/Game/Blueprints/Characters/BaseCharacterBP.Health` _asbase_character_bp)))))

(event `InputAction|DEBUG_KEY3`
  (params (Key :type "Key Structure"))
  ;[1 0.6118 0] DEBUG (Num Pad 3&4): Saves and Loads Party Subclasses
  (:`Pressed`
    (`/Game/Blueprints/MainGameModeBP.Save` (`self.GameModeRef`))))

(event `InputAction|DEBUG_KEY4`
  (params (Key :type "Key Structure"))
  ;[1 0.6118 0] DEBUG (Num Pad 3&4): Saves and Loads Party Subclasses
  (:`Pressed`
    (`/Game/Blueprints/MainGameModeBP.Load` (`self.GameModeRef`))))

(fn `ResetControlledPawn`
  ;[0 0 0] Resets ControlledPawn when a new pawn is possessed
  (set `self.ControlledCharacter` (`self.K2_GetPawn`)))

(fn `SwapCharacters`
  (params (NewIndex :type Integer))
  (locals (NewCharacter :type "/Game/Blueprints/Characters/PlayableCharacters/PlayableCharacterBP Object Reference") (PlayerController :type "PlayerController Object Reference") (NewCharacterIndex :type Integer))
  (bind _newcharacter (`local.NewCharacter`))
  (bind _gamemoderef (`self.GameModeRef`))
  ;[0 0 0] Preparation
  (`/Engine/EditorBlueprintResources/StandardMacros.IsValid` _gamemoderef
    (:`Is Valid`
      (bind _output_get (set `local.NewCharacterIndex` NewIndex))
      (set `local.NewCharacter` (`|GetArrayItem` (`/Game/Blueprints/MainGameModeBP.PlayableCharacters` _gamemoderef) _output_get))
      (set `local.PlayerController` (`GameplayStatics.GetPlayerController` 0))
      ;[0 0 0] Prevents swapping to already possessed character
      (if (!= (`self.K2_GetPawn` (`local.PlayerController`)) (`local.NewCharacter`))
        ;[0 0 0] Prevents swapping to KO's character
        (if (not (`/Game/Blueprints/Characters/PlayableCharacters/PlayableCharacterBP.KnockedOut` (`local.NewCharacter`)))
          ;[0 0 0] Swap
          (`self.Possess` (`local.PlayerController`) _newcharacter)
          ;;[0.5104 0.3754 0] Force a UI update; probably needs to be a separate function
          (`/Game/Blueprints/Characters/BaseCharacterBP.ReceiveHealthChange` _newcharacter 0)
          (bind _asplayer_controller_bp (cast `/Game/Blueprints/PlayerControllerBP` (`local.PlayerController`)))
          (`self.ResetControlledPawn` _asplayer_controller_bp)
          (set `/Game/Blueprints/MainGameModeBP.CurrentPlayableCharacterIndex` (`local.NewCharacterIndex`) (`self.GameModeRef`)))))))

(fn `UserConstructionScript`
  (bind _asmain_game_mode_bp (cast `/Game/Blueprints/MainGameModeBP` (`GameplayStatics.GetGameMode`)))
  (set `self.GameModeRef` _asmain_game_mode_bp))