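; Base actor component for status effects, such as those associated with pool actors, applied to the actor that owns it.
; BeginPlay calls ApplyStatusEffect, an empty hook for child effects to fill in.
; CheckIfInPool sets InPool when the owner overlaps a BasePoolBP whose StatusEffect class matches this component's own class.
; RemoveStatusEffect ends the effect by destroying the component.
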(event `self.ReceiveBeginPlay`
  (`self.ApplyStatusEffect`))

(fn `ApplyStatusEffect`)

(fn `CheckIfInPool`
  (set `self.InPool` false)
  (for _array_element (`Actor.GetOverlappingActors` (`self.GetOwner` self) "/Game/Blueprints/Spawnables/Pools/BasePoolBP.BasePoolBP_C")
    (if (== (`/Game/Blueprints/Spawnables/Pools/BasePoolBP.StatusEffect` (cast `/Game/Blueprints/Spawnables/Pools/BasePoolBP` _array_element :!pure true)) (`GameplayStatics.GetObjectClass` self))
      (set `self.InPool` true)
      (break)
      (else
        (set `self.InPool` false)))))

(fn `RemoveStatusEffect`
  (`self.K2_DestroyComponent`))