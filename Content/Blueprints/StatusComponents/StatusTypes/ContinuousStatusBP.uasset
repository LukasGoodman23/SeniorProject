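; Base-style status effect component for continuous effects that last until removed, then get undone.
; Each tick, pool-sourced effects call CheckIfInPool and end when no longer in the pool, while others count down LifetimeRemaining and end when it runs out.
; RemoveStatusEffect calls the empty UndoStatusEffect hook before the parent's removal logic; BeginPlay and ApplyStatusEffect simply defer to the parent.
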(event `self.ReceiveBeginPlay`
  (`parent.ReceiveBeginPlay`))

(event `self.ReceiveTick`
  (params (DeltaSeconds :type "Float (single-precision)"))
  (if (`self.FromPool`)
    ;[0 0 0] Pool Status
    (`self.CheckIfInPool`)
    (if (not (`self.InPool`))
      (`self.RemoveStatusEffect`))
    (else
      ;[0 0 0] Duration Status
      (bind _output_get (set `self.LifetimeRemaining` (- (`self.LifetimeRemaining`) DeltaSeconds)))
      (if (not (> _output_get 0.0))
        (`self.RemoveStatusEffect`)))))

(fn `ApplyStatusEffect`
  (`parent.ApplyStatusEffect`))

(fn `RemoveStatusEffect`
  (`self.UndoStatusEffect`)
  (`parent.RemoveStatusEffect`))

(fn `UndoStatusEffect`)