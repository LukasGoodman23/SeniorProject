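; Base-style status effect Blueprint that applies its effect on a repeating cooldown interval.
; Tick advances a timer and counts down the remaining lifetime; once the interval elapses, the effect reapplies while in a pool or while lifetime remains, otherwise it removes itself.
; Resetting subtracts the interval from the timer instead of zeroing it, carrying overshoot into the next interval.
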(event `self.ReceiveBeginPlay`
  (`parent.ReceiveBeginPlay`))

(event `self.ReceiveTick`
  (params (DeltaSeconds :type "Float (single-precision)"))
  ;[0 0 0] Tick timers
  ;;[0 0 0] Tick Timer
  (set `self.Timer` (+ DeltaSeconds (`self.Timer`)))
  (if (> (`self.LifetimeRemaining`) 0.0)
    (set `self.LifetimeRemaining` (- (`self.LifetimeRemaining`) DeltaSeconds))
    (if (< (`self.LifetimeRemaining`) 0.0)
      (set `self.LifetimeRemaining` 0.0)))
  ;[0 0 0] Check whether to remove or apply status on interval
  (if (>= (`self.Timer`) (`self.CooldownInterval`))
    ;;[0 0 0] Check if in a pool
    (bind _inpool (`self.CheckIfInPool`))
    (if _inpool
      (`self.ApplyStatusEffect`)
      (`self.ResetTimer`)
      (else
        ;;[0 0 0] If not in a pool, rely on lifetime
        (if (> (`self.LifetimeRemaining`) 0.0)
          (`self.ApplyStatusEffect`)
          (`self.ResetTimer`)
          (else
            (`self.RemoveStatusEffect`)))))))

(fn `ResetTimer`
  (set `self.Timer` (- (`self.Timer`) (`self.CooldownInterval`))))