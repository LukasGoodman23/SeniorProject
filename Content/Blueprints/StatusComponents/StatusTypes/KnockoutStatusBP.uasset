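; Knockout status component for playable characters that greys the status HUD and revives its owner when an automatic timer or manual revive timer completes.
; BeginPlay adds a visible capsule as revive range, registering overlapping same-affiliation characters so the owner becomes their interactable.
; Tick shows automatic progress on the health display and resets manual progress whenever ManualReviving is off.
; Removal unregisters allies, restores HUD color, calls Revive and destroys the component.
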(event `self.ReceiveBeginPlay`
  (bind _reviverange (`self.ReviveRange`))
  (`parent.ReceiveBeginPlay`)
  (set `self.TimerAutoGoal` (`self.LifetimeRemaining`))
  (bind _output_get (set `self.Owner` (cast `/Game/Blueprints/Characters/PlayableCharacters/PlayableCharacterBP` (`self.GetOwner`) :!pure true)))
  (bind _statushud (`/Game/Blueprints/Characters/PlayableCharacters/PlayableCharacterBP.StatusHUD` _output_get))
  (set `self.DefaultStatusColor` (`UserWidget.ColorAndOpacity` _statushud))
  (`UserWidget.SetColorAndOpacity` _statushud (struct :`R` 0.151042 :`G` 0.151042 :`B` 0.151042 :`A` 1.0))
  (bind _returnvalue (`|AddComponentByClass` (`self.GetOwner`) "/Script/Engine.CapsuleComponent" false (`KismetMathLibrary.MakeTransform` (0.0 0.0 0.0) (struct) (10.0 10.0 10.0))))
  (bind _output_get_2 (set `/Game/Blueprints/Characters/PlayableCharacters/PlayableCharacterBP.InteractionRadius` _returnvalue (`self.Owner`)))
  (bind _output_get_3 (set `self.ReviveRange` _output_get_2))
  (`SceneComponent.SetHiddenInGame` _output_get_3 false false)
  (`CapsuleComponent.SetCapsuleHalfHeight` _reviverange 0.0 true)
  (add `PrimitiveComponent.OnComponentBeginOverlap` _reviverange (delegate `ReviveRangeEntered`))
  (add `PrimitiveComponent.OnComponentEndOverlap` _reviverange (delegate `ReviveRangeExited`)))

(event `ReviveRangeEntered`
  (params (OverlappedComponent :type "PrimitiveComponent Object Reference") (OtherActor :type "Actor Object Reference") (OtherComp :type "PrimitiveComponent Object Reference") (OtherBodyIndex :type Integer) (bFromSweep :type Boolean) (SweepResult :type "HitResult Structure (by ref)"))
  ;[0 0 0] Probably not the way to do it. The character should probably be the one that checks to see if it's in the capsule, but this seems to work
  (bind _asbase_character_bp (cast `/Game/Blueprints/Characters/BaseCharacterBP` OtherActor))
  (if (`|EnumEquality` (`/Game/Blueprints/Characters/BaseCharacterBP.Affiliation` _asbase_character_bp) (`/Game/Blueprints/Characters/BaseCharacterBP.Affiliation` (`self.Owner`)))
    (`KismetArrayLibrary.Array_AddUnique` (`self.AlliesInRange`) _asbase_character_bp)
    (`KismetArrayLibrary.Array_AddUnique` (`/Game/Blueprints/Characters/BaseCharacterBP.InteractableCharacters` _asbase_character_bp) (`self.Owner`))))

(event `ReviveRangeExited`
  (params (OverlappedComponent :type "PrimitiveComponent Object Reference") (OtherActor :type "Actor Object Reference") (OtherComp :type "PrimitiveComponent Object Reference") (OtherBodyIndex :type Integer))
  ;[0 0 0] Probably not the way to do it. The character should probably be the one that checks to see if it's in the capsule, but this seems to work
  (bind _asbase_character_bp (cast `/Game/Blueprints/Characters/BaseCharacterBP` OtherActor))
  (if (== (`|GetArrayItem` (`/Game/Blueprints/Characters/BaseCharacterBP.InteractableCharacters` _asbase_character_bp)) (`self.Owner`))
    (`KismetArrayLibrary.Array_RemoveItem` (`self.AlliesInRange`) _asbase_character_bp)
    (`KismetArrayLibrary.Array_RemoveItem` (`/Game/Blueprints/Characters/BaseCharacterBP.InteractableCharacters` _asbase_character_bp) (`self.Owner`))))

(event `self.ReceiveTick`
  (params (DeltaSeconds :type "Float (single-precision)"))
  (if (not (`self.Paused`))
    (bind _output_get (set `self.TimerAutoProgress` (+ (`self.TimerAutoProgress`) DeltaSeconds)))
    (`/Game/Blueprints/Menus/StatusHUD.UpdateHealth` (`/Game/Blueprints/Characters/PlayableCharacters/PlayableCharacterBP.StatusHUD` (`self.Owner`)) (/ _output_get (`self.TimerAutoGoal`)))
    (if (`self.ManualReviving`)
      (set `self.TimerManualProgress` (+ (`self.TimerManualProgress`) DeltaSeconds))
      (else
        (set `self.TimerManualProgress` 0.0)))
    (if (or (>= (`self.TimerAutoProgress`) (`self.TimerAutoGoal`)) (>= (`self.TimerManualProgress`) (`self.TimerManualGoal`)))
      (`self.RemoveStatusEffect`))))

(fn `RemoveStatusEffect`
  (`parent.RemoveStatusEffect`)
  (for _array_element (`self.AlliesInRange`)
    (`KismetArrayLibrary.Array_RemoveItem` (`/Game/Blueprints/Characters/BaseCharacterBP.InteractableCharacters` _array_element) (`self.Owner`)))
  (`UserWidget.SetColorAndOpacity` (`/Game/Blueprints/Characters/PlayableCharacters/PlayableCharacterBP.StatusHUD` (`self.Owner`)) (`self.DefaultStatusColor`))
  (`/Game/Blueprints/Characters/BaseCharacterBP.Revive` (`self.Owner`))
  (`self.K2_DestroyComponent`))