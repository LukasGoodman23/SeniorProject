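; Slow status component that changes the walk speed of the BaseCharacterBP that owns it.
; ApplyStatusEffect calls the parent, then multiplies the character movement's MaxWalkSpeed by MovementSpeedMultiplier.
; UndoStatusEffect calls the parent, then divides by the same multiplier, reversing the change relative to the current speed instead of restoring a cached value.
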(fn `ApplyStatusEffect`
  (bind _charactermovement (`Character.CharacterMovement` (cast `/Game/Blueprints/Characters/BaseCharacterBP` (`self.GetOwner`) :!pure true)))
  (`parent.ApplyStatusEffect`)
  (set `CharacterMovementComponent.MaxWalkSpeed` (* (`CharacterMovementComponent.MaxWalkSpeed` _charactermovement) (`self.MovementSpeedMultiplier`)) _charactermovement))

(fn `UndoStatusEffect`
  (bind _charactermovement (`Character.CharacterMovement` (cast `/Game/Blueprints/Characters/BaseCharacterBP` (`self.GetOwner`) :!pure true)))
  (`parent.UndoStatusEffect`)
  (set `CharacterMovementComponent.MaxWalkSpeed` (/ (`CharacterMovementComponent.MaxWalkSpeed` _charactermovement) (`self.MovementSpeedMultiplier`)) _charactermovement))