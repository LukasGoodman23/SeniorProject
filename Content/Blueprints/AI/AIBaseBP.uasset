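; Base AI controller Blueprint that picks enemy targets by sight and mirrors its character's state to the Blackboard.
; Perception updates feed HandleSight, which, unless Attacked is set, stores any sight-sensed BaseCharacterBP of differing affiliation that isn't knocked out as EnemyActor.
; InitializeValues copies affiliation, health, knocked-out and stand-still values from the possessed pawn, and SetBlackboard writes them to keys.
; Neither setup function is called within this Blueprint.
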(event `self.AIPerception.OnTargetPerceptionUpdated`
  (params (Actor :type "Actor Object Reference") (Stimulus :type "AIStimulus Structure"))
  (`self.Handle Sight` Actor Stimulus)
  (`KismetSystemLibrary.Delay` 0.2))

(fn `Handle Sight`
  (params (Actor :type "Actor Object Reference") (Stimulus :type "AIStimulus Structure"))
  (bind _actor (`local.Actor`))
  (bind _asbase_character_bp (cast `/Game/Blueprints/Characters/BaseCharacterBP` _actor :!pure true))
  ;[0 0 0] If Actor is insight, and if that actor is of opposite affiliation, set as EnemyActor on Blackboard
  (if (`self.Attacked`)
    (return)
    (else
      (bind _returnvalue (`AIPerceptionSystem.GetSenseClassForStimulus` Stimulus))
      (if (== _returnvalue "/Script/AIModule.AISense_Sight")
        (`/Engine/EditorBlueprintResources/StandardMacros.IsValid` _actor
          (:`Is Valid`
            (`/Engine/EditorBlueprintResources/StandardMacros.IsValid` _asbase_character_bp
              (:`Is Valid`
                (if (`|EnumInequality` (`/Game/Blueprints/Characters/BaseCharacterBP.Affiliation` _asbase_character_bp) (`self.Affil`))
                  (if (!= (`/Game/Blueprints/Characters/BaseCharacterBP.KnockedOut` _asbase_character_bp) true)
                    (`BlackboardComponent.SetValueAsObject` (`self.Blackboard`) "EnemyActor" (`local.Actor`))
                    (else
                      (return)))
                  (else
                    (return))))
              (:`Is Not Valid`
                (return))))
          (:`Is Not Valid`
            (return)))
        (else
          (return))))))

(fn `Initialize Values`
  (params (`Possessed Pawn` :type "Pawn Object Reference"))
  ;[0 0 0] Takes Values from Character Blueprints
  (bind _asbase_character_bp (cast `/Game/Blueprints/Characters/BaseCharacterBP` `Possessed Pawn`))
  (set `self.Affil` (`/Game/Blueprints/Characters/BaseCharacterBP.Affiliation` _asbase_character_bp))
  (set `self.MaxHealth` (`/Game/Blueprints/Characters/BaseCharacterBP.MaxHealth` _asbase_character_bp))
  (set `self.Health` (`/Game/Blueprints/Characters/BaseCharacterBP.Health` _asbase_character_bp))
  (set `self.Dead` (`/Game/Blueprints/Characters/BaseCharacterBP.KnockedOut` _asbase_character_bp))
  (set `self.StandStill` (`/Game/Blueprints/Characters/BaseCharacterBP.StandStill` _asbase_character_bp)))

(fn `Set Blackboard`
  (bind _blackboard (`self.Blackboard`))
  ;[0 0 0] Setting CharacterBP Values to the Blackboard
  (`BlackboardComponent.SetValueAsEnum` _blackboard "Affil" (`self.Affil`))
  (`BlackboardComponent.SetValueAsInt` _blackboard "MaxHealth" (`self.MaxHealth`))
  (`BlackboardComponent.SetValueAsInt` _blackboard "CurrentHealth" (`self.Health`))
  (`BlackboardComponent.SetValueAsBool` _blackboard "IsDead" (`self.Dead`))
  (`BlackboardComponent.SetValueAsBool` _blackboard "StandStill" (`self.StandStill`)))

(fn `UserConstructionScript`)