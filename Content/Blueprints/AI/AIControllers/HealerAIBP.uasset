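; AI controller for the healer, which also announces the healer's arrival to the playable characters.
; On possession it runs HealerBT, initializes values from the possessed pawn, then calls HealerSummoned after a short delay.
; HealerSummoned loops over all PlayableCharacterBP actors and sets the "Healer" flag to true on each valid blackboard it finds.
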(event `self.ReceivePossess`
  (params (PossessedPawn :type "Pawn Object Reference"))
  (`self.RunBehaviorTree` "/Game/Blueprints/AI/BehaviorTrees/HealerBT.HealerBT")
  (`self.Initialize Values` PossessedPawn)
  (`KismetSystemLibrary.Delay` 0.1)
  (`self.HealerSummoned`))

(fn `HealerSummoned`
  (bind _outactors (`GameplayStatics.GetAllActorsOfClass` "/Game/Blueprints/Characters/PlayableCharacters/PlayableCharacterBP.PlayableCharacterBP_C"))
  (for _array_element _outactors
    (bind _returnvalue (`AIBlueprintHelperLibrary.GetBlackboard` _array_element))
    (`/Engine/EditorBlueprintResources/StandardMacros.IsValid` _returnvalue
      (:`Is Valid`
        (`BlackboardComponent.SetValueAsBool` _returnvalue "Healer" true)))))

(fn `UserConstructionScript`
  (`parent.UserConstructionScript`))