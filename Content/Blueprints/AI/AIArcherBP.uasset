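; AI controller for the archer that starts the ArcherBT behavior tree on possession.
; Perception updates pass to HandleSight, which writes sight-sensed actors of type BaseEnemyBP to the EnemyActor blackboard key.
; The successfully-sensed flag is not used, so losing sight does not clear that key.
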(event `self.ReceivePossess`
  (params (PossessedPawn :type "Pawn Object Reference"))
  (`self.RunBehaviorTree` "/Game/Blueprints/AI/BehaviorTrees/ArcherBT.ArcherBT")
  (`KismetSystemLibrary.PrintString` "Took Control of Archer"))

(event `self.AIPerception.OnTargetPerceptionUpdated`
  (params (Actor :type "Actor Object Reference") (Stimulus :type "AIStimulus Structure"))
  (`self.HandleSight` Actor Stimulus))

(fn `HandleSight`
  (params (Actor :type "Actor Object Reference") (Stimulus :type "AIStimulus Structure"))
  (bind _actor (`local.Actor`))
  (bind _returnvalue (`AIPerceptionSystem.GetSenseClassForStimulus` Stimulus))
  (if (== _returnvalue "/Script/AIModule.AISense_Sight")
    (if (== _actor (cast `/Game/Blueprints/Characters/Enemy/BaseEnemyBP` _actor :!pure true))
      (`BlackboardComponent.SetValueAsObject` (`self.Blackboard`) "EnemyActor" (`local.Actor`))
      (else
        (return)))
    (else
      (return))))

(fn `UserConstructionScript`)