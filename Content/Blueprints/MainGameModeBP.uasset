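; Game mode that manages a three-character party of knight, wizard and archer subclasses, with character switching and a game-over check.
; On BeginPlay it loads subclasses from a save slot or saves defaults, builds the party, then triggers the level's single PartySpawner.
; SpawnPlayableCharacters creates the characters, shared gameplay UI and camera; CycleCharacter possesses the next non-knocked-out member.
; Save writes hard-coded variant subclasses, and Load reopens the current level as a test.
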(event `self.ReceiveBeginPlay`
  (bind _returnvalue (`GameplayStatics.DoesSaveGameExist` "save1"))
  (if _returnvalue
    ;[0 0 0] If a game has been saved, load the saved character classes from slot1
    (bind _returnvalue_2 (`GameplayStatics.LoadGameFromSlot` "save1"))
    (bind _asbp_save_game (cast `/Game/Blueprints/Saving/BP_SaveGame` _returnvalue_2))
    (set `self.Save Game` _asbp_save_game)
    (set `self.KnightSubclass` (`/Game/Blueprints/Saving/BP_SaveGame.Knight Subclass` _asbp_save_game))
    (set `self.ArcherSubclass` (`/Game/Blueprints/Saving/BP_SaveGame.Archer Subclass` _asbp_save_game))
    (set `self.WizardSubclass` (`/Game/Blueprints/Saving/BP_SaveGame.Wizard Subclass` _asbp_save_game))
    (else
      ;[0 0 0] If no game has been saved, save the game with all subclass 1s to slot1
      (bind _returnvalue_3 (`GameplayStatics.CreateSaveGameObject` "/Game/Blueprints/Saving/BP_SaveGame.BP_SaveGame_C"))
      (`self.Save Subclasses` _returnvalue_3 "/Game/Blueprints/Characters/PlayableCharacters/CharacterClasses/KnightSubclasses/SubclassKnightVariant1.SubclassKnightVariant1_C" "/Game/Blueprints/Characters/PlayableCharacters/CharacterClasses/ArcherSubclasses/SubclassArcherVariant1.SubclassArcherVariant1_C" "/Game/Blueprints/Characters/PlayableCharacters/CharacterClasses/WizardSubclasses/HealingWizard.HealingWizard_C")
      (`GameplayStatics.SaveGameToSlot` _returnvalue_3 "save1")
      (set `self.Save Game` _returnvalue_3)))
  (`self.SetupParty`)
  (bind _outactors (`GameplayStatics.GetAllActorsOfClass` "/Game/Blueprints/Other/Spawners/PartySpawner.PartySpawner_C"))
  (bind _returnvalue_4 (`KismetArrayLibrary.Array_Length` _outactors))
  (if (== _returnvalue_4 1)
    (`/Game/Blueprints/Other/Spawners/PartySpawner.SpawnParty` (`|GetArrayItem` _outactors) :!label _label)
    (elif (> _returnvalue_4 1)
      (`KismetSystemLibrary.PrintString` (`KismetStringLibrary.BuildString_Int` "" "ISSUE: There are " _returnvalue_4 " PlayerSpawners in the world. \n     There cannot be more than 1.") true true (struct :`G` 0.66 :`B` 1.0 :`A` 1.0) 10.0)
      (goto _label)
      (else
        (`KismetSystemLibrary.PrintString` "There are no PlayerSpawners in the world. Please add one." true true (struct :`G` 0.66 :`B` 1.0 :`A` 1.0) 10.0)))))

(event `Save`
  (bind _save_game (`self.Save Game`))
  ;[0 0 0] Saves subclass 2s to slot1
  (bind _returnvalue (`GameplayStatics.DoesSaveGameExist` "save1"))
  (if _returnvalue
    (`self.Save Subclasses` _save_game "/Game/Blueprints/Characters/PlayableCharacters/CharacterClasses/KnightSubclasses/SubclassKnightVariant2.SubclassKnightVariant2_C" "/Game/Blueprints/Characters/PlayableCharacters/CharacterClasses/ArcherSubclasses/SubclassArcherVariant2.SubclassArcherVariant2_C" "/Game/Blueprints/Characters/PlayableCharacters/CharacterClasses/WizardSubclasses/SubclassWizardVariant2.SubclassWizardVariant2_C")
    (`GameplayStatics.SaveGameToSlot` _save_game "save1")))

(event `Load`
  (bind _save_game (`self.Save Game`))
  ;[0 0 0] Loads the game from save1 (currently reopens whatever level is currently running)
  (bind _returnvalue (`GameplayStatics.DoesSaveGameExist` "save1"))
  (if _returnvalue
    (set `self.KnightSubclass` (`/Game/Blueprints/Saving/BP_SaveGame.Knight Subclass` _save_game))
    (set `self.ArcherSubclass` (`/Game/Blueprints/Saving/BP_SaveGame.Archer Subclass` _save_game))
    (set `self.WizardSubclass` (`/Game/Blueprints/Saving/BP_SaveGame.Wizard Subclass` _save_game))
    ;;[1 0.6118 0] TESTING
    (bind _returnvalue_2 (`GameplayStatics.GetCurrentLevelName` true))
    (`GameplayStatics.OpenLevel` (`KismetStringLibrary.Conv_StringToName` _returnvalue_2))))

(fn `CheckForGameOver`
  (returns (GameOver :type Boolean))
  (locals (KnockedOutCount :type Integer))
  (for _array_element (`self.PlayableCharacters`)
    (if (`/Game/Blueprints/Characters/BaseCharacterBP.KnockedOut` _array_element)
      (`/Engine/EditorBlueprintResources/StandardMacros.IncrementInt` (`local.KnockedOutCount`))))
  (return (>= (`local.KnockedOutCount`) (`KismetArrayLibrary.Array_Length` (`self.PlayableCharacters`)))))

(fn `Cycle Character`
  (params (Controller :type "/Game/Blueprints/PlayerControllerBP Object Reference"))
  (locals (CheckedCharacters :type Integer :default 0) (CharacterAvailable :type Boolean) (PlayerController :type "/Game/Blueprints/PlayerControllerBP Object Reference") (OldActiveCharacter :type "/Game/Blueprints/Characters/PlayableCharacters/PlayableCharacterBP Object Reference") (NewActiveCharacter :type "/Game/Blueprints/Characters/PlayableCharacters/PlayableCharacterBP Object Reference"))
  (bind _playercontroller (`local.PlayerController`))
  (set `local.PlayerController` Controller)
  (set `self.OldCharacterIndex` (`self.CurrentPlayableCharacterIndex`))
  (if (> (`KismetArrayLibrary.Array_Length` (`self.PlayableCharacters`)) 0)
    ;[0 0 0] Increment index
    ;;[0 0 0] Continue checking for an available character
    (while (and (not (`local.CharacterAvailable`)) (< (`local.CheckedCharacters`) (`KismetArrayLibrary.Array_Length` (`self.PlayableCharacters`))))
      (bind _result (`/Engine/EditorBlueprintResources/StandardMacros.IncrementInt` (`self.CurrentPlayableCharacterIndex`))
        (:`  `
          (if (>= _result (`KismetArrayLibrary.Array_Length` (`self.PlayableCharacters`)))
            (set `self.CurrentPlayableCharacterIndex` 0))
          (`/Engine/EditorBlueprintResources/StandardMacros.IncrementInt` (`local.CheckedCharacters`)
            (:`  `
              (if (not (`/Game/Blueprints/Characters/PlayableCharacters/PlayableCharacterBP.KnockedOut` (`|GetArrayItem` (`self.PlayableCharacters`) (`self.CurrentPlayableCharacterIndex`))))
                (set `local.CharacterAvailable` true)))))))
    ;[0 0 0] Possession
    ;;[0 0 0] Prevents repossessing already possessed character
    (if (< (`local.CheckedCharacters`) (`KismetArrayLibrary.Array_Length` (`self.PlayableCharacters`)))
      (bind _output_get (set `local.OldActiveCharacter` (cast `/Game/Blueprints/Characters/PlayableCharacters/PlayableCharacterBP` (`/Game/Blueprints/PlayerControllerBP.ControlledCharacter` _playercontroller) :!pure true)))
      (set `/Game/Blueprints/Characters/PlayableCharacters/PlayableCharacterBP.Possessed` false _output_get)
      (bind _output_get_2 (set `local.NewActiveCharacter` (`|GetArrayItem` (`self.PlayableCharacters`) (`self.CurrentPlayableCharacterIndex`))))
      (set `/Game/Blueprints/Characters/PlayableCharacters/PlayableCharacterBP.Possessed` true _output_get_2)
      (`Controller.Possess` _playercontroller _output_get_2)
      (`/Game/Blueprints/PlayerControllerBP.ResetControlledPawn` _playercontroller)
      (`/Game/Blueprints/Menus/Widgets/GameplayUI.Swap Character` (`self.GameplayUI`) (`self.OldCharacterIndex`) (`self.CurrentPlayableCharacterIndex`))
      (`/Game/Blueprints/CameraBP.SetCharacterView` (`/Game/Blueprints/PlayerControllerBP.CameraObject` (`local.PlayerController`)) (`local.NewActiveCharacter`))
      (set `self.OldCharacterIndex` (`self.CurrentPlayableCharacterIndex`)))))

(fn `Save Subclasses`
  (params (Save :type "/Game/Blueprints/Saving/BP_SaveGame Object Reference") (Knight :type "/Game/Blueprints/Characters/PlayableCharacters/CharacterClasses/ClassKnightBP Class Reference") (Archer :type "/Game/Blueprints/Characters/PlayableCharacters/CharacterClasses/ClassArcherBP Class Reference") (Wizard :type "/Game/Blueprints/Characters/PlayableCharacters/CharacterClasses/ClassWizardBP Class Reference"))
  (set `/Game/Blueprints/Saving/BP_SaveGame.Knight Subclass` Knight Save)
  (set `/Game/Blueprints/Saving/BP_SaveGame.Archer Subclass` Archer Save)
  (set `/Game/Blueprints/Saving/BP_SaveGame.Wizard Subclass` Wizard Save))

(fn `SetupParty`
  (`KismetArrayLibrary.Array_Clear` (`self.Party`))
  (`KismetArrayLibrary.Array_Add` (`self.Party`) (`self.KnightSubclass`))
  (`KismetArrayLibrary.Array_Add` (`self.Party`) (`self.WizardSubclass`))
  (`KismetArrayLibrary.Array_Add` (`self.Party`) (`self.ArcherSubclass`)))

(fn `SpawnPlayableCharacters`
  (params (SpawnLocations :type "Array of Vector Structure"))
  (bind _gameplayui (`self.GameplayUI`))
  (bind _gameplayui_2 (`self.GameplayUI`))
  (bind _asplayer_controller_bp (cast `/Game/Blueprints/PlayerControllerBP` (`GameplayStatics.GetPlayerController` 0) :!pure true))
  (bind _output (`|GetArrayItem` (`self.PlayableCharacters`)))
  ;[0 0 0] Spawn playable characters into the level
  (bind _returnvalue (`|GenericCreateObject` "/Game/Blueprints/Menus/Widgets/GameplayUI.GameplayUI_C"))
  (set `self.GameplayUI` _returnvalue)
  (`KismetArrayLibrary.Array_Clear` (`self.PlayableCharacters`))
  (for (_array_element _array_index) SpawnLocations
    (bind _returnvalue_2 (`|SpawnActorFromClass` (`|GetArrayItem` (`self.Party`) _array_index) (`KismetMathLibrary.MakeTransform` _array_element) "AdjustIfPossibleButAlwaysSpawn" "OverrideRootScale" null null))
    (`KismetArrayLibrary.Array_Add` (`self.PlayableCharacters`) _returnvalue_2)
    (`KismetArrayLibrary.Array_Add` (`/Game/Blueprints/Menus/Widgets/GameplayUI.Characters` _gameplayui) _returnvalue_2)
    (set `/Game/Blueprints/Characters/PlayableCharacters/PlayableCharacterBP.GameplayUI` _gameplayui _returnvalue_2))
  (`UserWidget.AddToViewport` _gameplayui_2 0)
  (`/Game/Blueprints/Menus/Widgets/GameplayUI.Construct Statuses` _gameplayui_2)
  ;;[0 0 0] Possess the first character
  (`Controller.Possess` (`GameplayStatics.GetPlayerController` 0) _output)
  (bind _returnvalue_3 (`|SpawnActorFromClass` "/Game/Blueprints/CameraBP.CameraBP_C" (`SceneComponent.K2_GetComponentToWorld` (`/Game/Blueprints/Characters/PlayableCharacters/PlayableCharacterBP.CameraLocationReference` _output)) "Undefined" "OverrideRootScale" null _asplayer_controller_bp null))
  (bind _output_get (set `/Game/Blueprints/PlayerControllerBP.CameraObject` _returnvalue_3 _asplayer_controller_bp))
  (`/Game/Blueprints/CameraBP.InitializeView` _output_get _output))

(fn `UserConstructionScript`)