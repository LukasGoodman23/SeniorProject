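; Camera actor that follows a viewed character, with a tilt-shift look from depth-of-field settings whose focal distance updates every tick to the camera-to-spring-arm distance.
; InitializeView attaches it to the character's camera reference, makes it the view target and clamps camera pitch relative to that character's transform.
; SetCharacterView switches characters, lerping between transforms on a sinusoidal timeline while camera control is locked for half a second.
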(event `self.ReceiveBeginPlay`
  ;[0 0 0] Tilt Shift
  (setmembers `PostProcessSettings` :`StructRef` (`PostProcessComponent.Settings` (`self.PostProcess`)) :`DepthOfFieldFstop` 0.25 :`DepthOfFieldSensorWidth` 75.0 :`DepthOfFieldFocalDistance` (`SpringArmComponent.TargetArmLength` (`self.SpringArm`))))

(event `self.ReceiveTick`
  (params (DeltaSeconds :type "Float (single-precision)"))
  ;[0 0 0] Tilt Shift
  (setmembers `PostProcessSettings` :`StructRef` (`PostProcessComponent.Settings` (`self.PostProcess`)) :`DepthOfFieldFstop` 0.25 :`DepthOfFieldSensorWidth` 75.0 :`DepthOfFieldFocalDistance` (`KismetMathLibrary.VSize` (- (`SceneComponent.K2_GetComponentLocation` (`self.Camera`)) (`SceneComponent.K2_GetComponentLocation` (`self.SpringArm`))))))

(event `InitializeView`
  (params (StartingCharacter :type "/Game/Blueprints/Characters/PlayableCharacters/PlayableCharacterBP Object Reference"))
  (bind _returnvalue (`GameplayStatics.GetPlayerCameraManager` 0))
  (bind _returnvalue_2 (* (.pitch (.rotation (`SceneComponent.K2_GetComponentToWorld` (`/Game/Blueprints/Characters/PlayableCharacters/PlayableCharacterBP.TransformationReference` (`self.CharacterViewing`))))) -1.0))
  (`self.K2_AttachToComponent` (`/Game/Blueprints/Characters/PlayableCharacters/PlayableCharacterBP.CameraLocationReference` StartingCharacter) "None" "KeepRelative" "KeepRelative" "KeepRelative")
  (set `self.CharacterViewing` StartingCharacter)
  (`PlayerController.SetViewTargetWithBlend` (`GameplayStatics.GetPlayerController` 0) self 0.0 "VTBlend_Linear" 0.0 false)
  (`self.K2_SetActorTransform` (`SceneComponent.K2_GetComponentToWorld` (`/Game/Blueprints/Characters/PlayableCharacters/PlayableCharacterBP.TransformationReference` (`self.CharacterViewing`))))
  ;[0 0 0] Clamp horizontal camera rotation
  (set `PlayerCameraManager.ViewPitchMin` (+ _returnvalue_2 -60.0) _returnvalue)
  (set `PlayerCameraManager.ViewPitchMax` (+ _returnvalue_2 5.0) _returnvalue))

(event `SetCharacterView`
  (params (Character :type "/Game/Blueprints/Characters/PlayableCharacters/PlayableCharacterBP Object Reference"))
  (set `self.PreviousLocation` (`SceneComponent.K2_GetComponentToWorld` (`self.SpringArm`)))
  (`self.K2_DetachFromActor` "KeepRelative")
  (`self.K2_AttachToComponent` (`/Game/Blueprints/Characters/PlayableCharacters/PlayableCharacterBP.CameraLocationReference` Character) "None" "KeepRelative" "KeepRelative" "KeepRelative")
  (set `self.CharacterViewing` Character)
  (`PlayerController.SetViewTargetWithBlend` (`GameplayStatics.GetPlayerController` 0) self 0.0 "VTBlend_Linear" 0.0 false)
  (`self.CameraTransition`)
  (set `/Game/Blueprints/PlayerControllerBP.LockCameraControl` true (`self.Controller`))
  (`KismetSystemLibrary.Delay` 0.5)
  (set `/Game/Blueprints/PlayerControllerBP.LockCameraControl` false (`self.Controller`))
  (set `self.PreviousLocation` (struct)))

(event `CameraTransition`
  ;[0 0 0] LERPs the camera from its current position to the next position
  (bind (_direction _cameratransition) (`Timeline|SinusoidalCameraTransitionTimeline` :!via `PlayFromStart`)
    (:`Update`
      (`self.K2_SetActorTransform` (`KismetMathLibrary.TLerp` (`self.PreviousLocation`) (`SceneComponent.K2_GetComponentToWorld` (`/Game/Blueprints/Characters/PlayableCharacters/PlayableCharacterBP.TransformationReference` (`self.CharacterViewing`))) _cameratransition)))))

(fn `UserConstructionScript`)