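; EnemyBarrierBP is a barrier actor that opens once its linked enemy spawner area is cleared.
; Tick polls the SpawnerArea's AreaCleared flag and calls Open while the barrier is still closed.
; Polling keeps spawners independent of barriers, with the tick interval slowed to one second to limit cost.
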(event `self.ReceiveTick`
  (params (DeltaSeconds :type "Float (single-precision)"))
  (`parent.ReceiveTick` DeltaSeconds)
  ;[1 0.7891 0] Probably shouldn't be on Tick, but I can't think of a better way right now (I don't want the spawner to call on this directly, because I want spawners to be independent from barriers)
  ; For the time being, this actor's tick has been made to be 1.0 second
  ; ~Wesley
  (if (and (not (`self.IsOpen`)) (`/Game/Blueprints/Other/Spawners/EnemySpawnerAreaManagerBP.AreaCleared` (`self.SpawnerArea`)))
    (`self.Open`)))

(fn `UserConstructionScript`
  (`parent.UserConstructionScript`))