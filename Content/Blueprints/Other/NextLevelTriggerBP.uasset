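; Level-end trigger that moves the game on when the player passes through its box.
; An overlap counts only for the controlled character's hurtbox and fires once, adding a fade-to-black widget.
; After a delay it saves NextLevel through the game mode, then opens either CharacterSelect or Credits based on ReturnToCharacterSelect, rather than loading NextLevel directly.
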(event `self.Box.OnComponentBeginOverlap`
  (params (OverlappedComponent :type "PrimitiveComponent Object Reference") (OtherActor :type "Actor Object Reference") (OtherComp :type "PrimitiveComponent Object Reference") (OtherBodyIndex :type Integer) (bFromSweep :type Boolean) (SweepResult :type "HitResult Structure (by ref)"))
  ;[0 0 0] Check to make sure the player passed through
  (bind _asplayable_character_bp (cast `/Game/Blueprints/Characters/PlayableCharacters/PlayableCharacterBP` OtherActor))
  (if (and (== (`/Game/Blueprints/Characters/BaseCharacterBP.Hurtbox` _asplayable_character_bp) OtherComp) (== _asplayable_character_bp (`/Game/Blueprints/PlayerControllerBP.ControlledCharacter` (cast `/Game/Blueprints/PlayerControllerBP` (`GameplayStatics.GetPlayerController` 0) :!pure true))))
    (`/Engine/EditorBlueprintResources/StandardMacros.DoOnce` false
      (:`Completed`
        ;[0 0 0] Transition
        (bind _returnvalue (`|CreateWidget` "/Game/Blueprints/Menus/Widgets/Popups/FadeToBlackBP.FadeToBlackBP_C"))
        (`UserWidget.AddToViewport` _returnvalue 1)
        (`KismetSystemLibrary.Delay` 5.0)
        (`/Game/Blueprints/MainGameModeBP.SetSaveLevel` (cast `/Game/Blueprints/MainGameModeBP` (`GameplayStatics.GetGameMode`) :!pure true) (`self.NextLevel`))
        (if (`self.ReturnToCharacterSelect`)
          (`GameplayStatics.OpenLevel` "CharacterSelect")
          (else
            (`GameplayStatics.OpenLevel` "Credits")))))))

(fn `UserConstructionScript`)