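; HealingPickupBP is a pickup that restores HealthAmount health to the character triggering it.
; It overrides the parent's PickupCondition to accept only characters below max health who are not knocked out, and PickupEffect to apply the heal.
; On BeginPlay it spawns and attaches a ParticlePersistenceBP running the TrailMagic effect, passing itself as LifetimeBoundCreator.
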(event `self.ReceiveBeginPlay`
  (`parent.ReceiveBeginPlay`)
  (bind _returnvalue (`|SpawnActorFromClass` "/Game/Niagara/ParticlePersistenceBP.ParticlePersistenceBP_C" (`self.GetTransform`) "Undefined" "OverrideRootScale" self "/Game/Niagara/Trail/TrailMagic.TrailMagic" self null))
  (bind _output_get (set `self.ParticleSystem` _returnvalue))
  (`self.K2_AttachToActor` _output_get self "None" "KeepWorld" "KeepWorld" "KeepWorld" true))

(fn `PickupCondition`
  (params (TriggeringCharacter :type "/Game/Blueprints/Characters/PlayableCharacters/PlayableCharacterBP Object Reference"))
  (returns (CanBePickedUp :type Boolean))
  (locals (Character :type "/Game/Blueprints/Characters/PlayableCharacters/PlayableCharacterBP Object Reference"))
  (bind _character (`local.Character`))
  (set `local.Character` TriggeringCharacter)
  (return (and (< (`/Game/Blueprints/Characters/BaseCharacterBP.Health` _character) (`/Game/Blueprints/Characters/BaseCharacterBP.MaxHealth` _character)) (not (`/Game/Blueprints/Characters/BaseCharacterBP.KnockedOut` _character)))))

(fn `PickupEffect`
  (params (TriggeringCharacter :type "/Game/Blueprints/Characters/PlayableCharacters/PlayableCharacterBP Object Reference"))
  (locals (Character :type "/Game/Blueprints/Characters/PlayableCharacters/PlayableCharacterBP Object Reference"))
  (bind _output_get (set `local.Character` TriggeringCharacter))
  (`parent.PickupEffect` _output_get)
  (`/Game/Blueprints/Characters/BaseCharacterBP.ReceiveDeltaHealth` _output_get (`self.HealthAmount`) self))

(fn `UserConstructionScript`
  (`parent.UserConstructionScript`))