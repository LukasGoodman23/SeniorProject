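; Area manager that owns a ring of enemy spawners and tracks when the area is cleared.
; MakeSpawnPoints destroys old spawners, then spawns and attaches new ones evenly around the actor at a set radius, facing inward, each referencing the manager.
; BeginSpawning triggers every spawner, while ClearedSpawner counts finished spawners and, once all are done, flags the area cleared and calls Cleared.
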(fn `BeginSpawning`
  (for _array_element (`self.EnemySpawners`)
    (`/Game/Blueprints/Other/Spawners/EnemySpawner.SpawnEnemies` _array_element)))

(fn `ClearedSpawner`
  (`/Engine/EditorBlueprintResources/StandardMacros.IncrementInt` (`self.ClearedSpawnersCount`)
    (:`  `
      (if (>= (`self.ClearedSpawnersCount`) (`self.SpawnerCount`))
        (set `self.AreaCleared` true)
        (`self.Cleared`)))))

(fn `MakeSpawnPoints`
  (locals (SpawnerCountTracker :type Integer :default 0) (Angle :type "Float (double-precision)") (DeltaAngle :type "Float (double-precision)") (Radius :type "Float (double-precision)" :default 500.0))
  (bind (_returnvalue_roll _returnvalue_pitch _returnvalue_yaw) (`KismetMathLibrary.BreakRotator` (`self.K2_GetActorRotation` self)))
  (bind _returnvalue_location (`KismetMathLibrary.BreakTransform` (`self.GetTransform` self)))
  ;[0 0 0] Reset if spawners already exist
  (for _array_element (`self.EnemySpawners`)
    (`self.K2_DestroyActor` _array_element))
  (`KismetArrayLibrary.Array_Clear` (`self.EnemySpawners`))
  (bind _output_get (set `local.SpawnerCountTracker` (`self.SpawnerCount`)))
  (if (!= _output_get 0)
    (set `local.DeltaAngle` (/ 360.0 (`KismetMathLibrary.Conv_IntToDouble` _output_get)))
    (set `local.Angle` _returnvalue_yaw)
    (while (> (`local.SpawnerCountTracker`) 0)
      (`/Engine/EditorBlueprintResources/StandardMacros.DecrementInt` (`local.SpawnerCountTracker`)
        (:`  `
          ;[0 0 0] Create Spawn Point
          (bind _returnvalue (`|SpawnActorFromClass` "/Game/Blueprints/Other/Spawners/EnemySpawner.EnemySpawner_C" (`KismetMathLibrary.MakeTransform` (+ (* (`KismetMathLibrary.GetForwardVector` (`KismetMathLibrary.MakeRotator` 0.0 0.0 (`local.Angle`))) (`local.Radius`)) _returnvalue_location) (`KismetMathLibrary.MakeRotator` 0.0 0.0 (- (`local.Angle`) 180.0))) "AlwaysSpawn" "OverrideRootScale" null self null))
          (`KismetArrayLibrary.Array_Add` (`self.EnemySpawners`) _returnvalue)
          (`self.K2_AttachToActor` _returnvalue self "None" "KeepWorld" "KeepWorld" "KeepWorld" true)
          (set `local.Angle` (+ (`local.Angle`) (`local.DeltaAngle`))))))))

(fn `UserConstructionScript`)