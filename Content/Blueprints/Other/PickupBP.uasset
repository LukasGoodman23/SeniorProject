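; Base pickup actor that a playable character collects by touching it, with the effect left empty for child Blueprints.
; It becomes active shortly after BeginPlay, then responds to Hitbox overlaps only when the character's Hurtbox touches it.
; PickupCondition gates collection and returns false by default.
; When the condition passes, PickupEffect runs on that character and the pickup destroys itself.
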(event `self.ReceiveBeginPlay`
  (`KismetSystemLibrary.Delay` 0.2)
  (set `self.Active` true))

(event `self.ReceiveActorBeginOverlap`
  (params (OtherActor :type "Actor Object Reference")))

(event `self.Hitbox.OnComponentBeginOverlap`
  (params (OverlappedComponent :type "PrimitiveComponent Object Reference") (OtherActor :type "Actor Object Reference") (OtherComp :type "PrimitiveComponent Object Reference") (OtherBodyIndex :type Integer) (bFromSweep :type Boolean) (SweepResult :type "HitResult Structure (by ref)"))
  (if (`self.Active`)
    (bind _asplayable_character_bp (cast `/Game/Blueprints/Characters/PlayableCharacters/PlayableCharacterBP` OtherActor))
    (if (`PrimitiveComponent.IsOverlappingComponent` (`/Game/Blueprints/Characters/BaseCharacterBP.Hurtbox` _asplayable_character_bp) OverlappedComponent)
      (bind _canbepickedup (`self.PickupCondition` _asplayable_character_bp))
      (if _canbepickedup
        (`self.PickupEffect` _asplayable_character_bp)
        (`self.K2_DestroyActor`)))))

(fn `PickupCondition`
  (params (TriggeringCharacter :type "/Game/Blueprints/Characters/PlayableCharacters/PlayableCharacterBP Object Reference"))
  (returns (CanBePickedUp :type Boolean))
  (return false))

(fn `PickupEffect`
  (params (TriggeringCharacter :type "/Game/Blueprints/Characters/PlayableCharacters/PlayableCharacterBP Object Reference")))

(fn `UserConstructionScript`)