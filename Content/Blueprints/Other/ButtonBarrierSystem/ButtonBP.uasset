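; ButtonBP is a pressure button in a button-barrier system that notifies its OwningBarrier when pressed or released.
; Overlaps with a playable character's Hurtbox maintain the OnButton list, pressing on entry if not already pressed.
; With HoldButton set, it releases once the list empties; otherwise it stays pressed.
; Material swaps show button type and pressed state, with the construction script setting the initial look.
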(event `self.ReceiveBeginPlay`)

(event `self.TEMP.OnComponentBeginOverlap`
  (params (OverlappedComponent :type "PrimitiveComponent Object Reference") (OtherActor :type "Actor Object Reference") (OtherComp :type "PrimitiveComponent Object Reference") (OtherBodyIndex :type Integer) (bFromSweep :type Boolean) (SweepResult :type "HitResult Structure (by ref)"))
  (bind _asplayable_character_bp (cast `/Game/Blueprints/Characters/PlayableCharacters/PlayableCharacterBP` OtherActor))
  (if (== (`/Game/Blueprints/Characters/BaseCharacterBP.Hurtbox` _asplayable_character_bp) OtherComp)
    (`KismetArrayLibrary.Array_AddUnique` (`self.OnButton`) _asplayable_character_bp)
    (if (not (`self.Pressed`))
      (`self.Press`))))

(event `self.TEMP.OnComponentEndOverlap`
  (params (OverlappedComponent :type "PrimitiveComponent Object Reference") (OtherActor :type "Actor Object Reference") (OtherComp :type "PrimitiveComponent Object Reference") (OtherBodyIndex :type Integer))
  (bind _onbutton (`self.OnButton`))
  (bind _asplayable_character_bp (cast `/Game/Blueprints/Characters/PlayableCharacters/PlayableCharacterBP` OtherActor))
  (if (== (`/Game/Blueprints/Characters/BaseCharacterBP.Hurtbox` _asplayable_character_bp) OtherComp)
    (`KismetArrayLibrary.Array_RemoveItem` _onbutton _asplayable_character_bp)
    (if (and (<= (`KismetArrayLibrary.Array_Length` _onbutton) 0) (`self.HoldButton`))
      (`self.Release`))))

(fn `Press`
  (set `self.Pressed` true)
  (`/Game/Blueprints/Other/ButtonBarrierSystem/ButtonBarrierBP.ButtonPressed` (`self.OwningBarrier`))
  (if (`self.HoldButton`)
    (`PrimitiveComponent.SetMaterial` (`self.TEMP`) 0 "/Game/TEMPMaterials/PurpleWizard.PurpleWizard")
    (else
      (`PrimitiveComponent.SetMaterial` (`self.TEMP`) 0 "/Game/TEMPMaterials/GreenArcher.GreenArcher"))))

(fn `Release`
  (set `self.Pressed` false)
  (`/Game/Blueprints/Other/ButtonBarrierSystem/ButtonBarrierBP.ButtonReleased` (`self.OwningBarrier`))
  (if (`self.HoldButton`)
    (`PrimitiveComponent.SetMaterial` (`self.TEMP`) 0 "/Game/TEMPMaterials/RedKnight.RedKnight")))

(fn `UserConstructionScript`
  (`SceneComponent.SetAbsolute` (`self.DefaultSceneRoot`) true true true)
  (if (`self.HoldButton`)
    (`PrimitiveComponent.SetMaterial` (`self.TEMP`) 0 "/Game/TEMPMaterials/RedKnight.RedKnight")
    (else
      (`PrimitiveComponent.SetMaterial` (`self.TEMP`) 0 "/Game/TEMPMaterials/BlueWizard.BlueWizard"))))