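; ButtonBarrierBP is a barrier that opens once enough of its linked buttons are pressed and closes when too few remain pressed.
; MakeButtons rebuilds an evenly spaced ring of attached ButtonBP actors around the barrier, each owned by it, with the threshold set to their count.
; Press and release calls update the tally, toggling the mesh's visibility and collision.
; With CannotClose set, opening force-presses every button with HoldButton off.
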(fn `ButtonPressed`
  (`/Engine/EditorBlueprintResources/StandardMacros.IncrementInt` (`self.PressedButtons`)
    (:`  `
      (if (and (>= (`self.PressedButtons`) (`self.ButtonThreshhold`)) (not (`self.IsOpen`)))
        (`self.Open`)))))

(fn `ButtonReleased`
  (`/Engine/EditorBlueprintResources/StandardMacros.DecrementInt` (`self.PressedButtons`)
    (:`  `
      (if (< (`self.PressedButtons`) (`self.ButtonThreshhold`))
        (`self.Close`)))))

(fn `Close`
  (bind _tempmesh (`self.TempMesh`))
  (`parent.Close`)
  ;[0 0 0] Close Visuals
  (`SceneComponent.SetVisibility` _tempmesh true false)
  (`PrimitiveComponent.SetCollisionResponseToAllChannels` _tempmesh "ECR_Block"))

(fn `MakeButtons`
  (locals (ButtonCountTracker :type Integer) (Angle :type "Float (double-precision)") (DeltaAngle :type "Float (double-precision)") (Radius :type "Float (double-precision)" :default 500.0))
  (bind _buttoncount (`self.ButtonCount`))
  (bind (_returnvalue_roll _returnvalue_pitch _returnvalue_yaw) (`KismetMathLibrary.BreakRotator` (`self.K2_GetActorRotation` self)))
  (bind _returnvalue_location (`KismetMathLibrary.BreakTransform` (`self.GetTransform` self)))
  ;[0 0 0] Reset if buttons already exist
  (for _array_element (`self.Buttons`)
    (`self.K2_DestroyActor` _array_element))
  (`KismetArrayLibrary.Array_Clear` (`self.Buttons`))
  (set `self.ButtonThreshhold` _buttoncount)
  (bind _output_get (set `local.ButtonCountTracker` _buttoncount))
  (if (!= _output_get 0)
    (set `local.DeltaAngle` (/ 360.0 (`KismetMathLibrary.Conv_IntToDouble` _output_get)))
    (set `local.Angle` _returnvalue_yaw)
    (while (> (`local.ButtonCountTracker`) 0)
      (`/Engine/EditorBlueprintResources/StandardMacros.DecrementInt` (`local.ButtonCountTracker`)
        (:`  `
          ;[0 0 0] Create Button
          (bind _returnvalue (`|SpawnActorFromClass` "/Game/Blueprints/Other/ButtonBarrierSystem/ButtonBP.ButtonBP_C" (`KismetMathLibrary.MakeTransform` (+ (* (`KismetMathLibrary.GetForwardVector` (`KismetMathLibrary.MakeRotator` 0.0 0.0 (`local.Angle`))) (`local.Radius`)) _returnvalue_location)) "AdjustIfPossibleButAlwaysSpawn" "OverrideRootScale" null self true null))
          (`KismetArrayLibrary.Array_Add` (`self.Buttons`) _returnvalue)
          (`self.K2_AttachToActor` _returnvalue self "None" "KeepWorld" "KeepWorld" "KeepWorld" true)
          (set `local.Angle` (+ (`local.Angle`) (`local.DeltaAngle`))))))))

(fn `Open`
  (bind _tempmesh (`self.TempMesh`))
  (`parent.Open`)
  ;[0 0 0] Open Visuals
  (`SceneComponent.SetVisibility` _tempmesh false false)
  (`PrimitiveComponent.SetCollisionResponseToAllChannels` _tempmesh "ECR_Ignore")
  (if (`self.CannotClose`)
    (for _array_element (`self.Buttons`)
      (set `/Game/Blueprints/Other/ButtonBarrierSystem/ButtonBP.HoldButton` false _array_element)
      (`/Game/Blueprints/Other/ButtonBarrierSystem/ButtonBP.Press` _array_element))))

(fn `UserConstructionScript`
  (`parent.UserConstructionScript`))