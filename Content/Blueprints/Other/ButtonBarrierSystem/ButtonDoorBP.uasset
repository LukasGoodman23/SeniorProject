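; ButtonDoorBP is a double swinging door in the button barrier system, overriding Open from its parent class.
; Open plays the SwingOpen timeline from the start, whose track yaws Cylinder and Cylinder1 in opposite directions, scaled to a quarter turn each.
; The parent Open call is left unconnected, so only the swing runs, and the graph has no closing logic.
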(fn `Open`
  (`TimelineComponent.PlayFromStart` (`self.SwingOpen`)))

(fn `UserConstructionScript`
  (`parent.UserConstructionScript`))