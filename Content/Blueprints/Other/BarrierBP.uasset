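; BarrierBP is a toggleable barrier actor that either blocks or lets things pass.
; On BeginPlay it applies its initial IsOpen state by calling Open or Close.
; Close shows the TEMP component and sets the Barrier collision to block all channels.
; Open hides TEMP in game and sets Barrier to overlap all channels, with both functions updating IsOpen.
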(event `self.ReceiveBeginPlay`
  (if (`self.IsOpen`)
    (`self.Open`)
    (else
      (`self.Close`))))

(fn `Close`
  (set `self.IsOpen` false)
  (`SceneComponent.SetHiddenInGame` (`self.TEMP`) false false)
  (`PrimitiveComponent.SetCollisionResponseToAllChannels` (`self.Barrier`) "ECR_Block"))

(fn `Open`
  (set `self.IsOpen` true)
  (`SceneComponent.SetHiddenInGame` (`self.TEMP`) true false)
  (`PrimitiveComponent.SetCollisionResponseToAllChannels` (`self.Barrier`) "ECR_Overlap"))

(fn `UserConstructionScript`)