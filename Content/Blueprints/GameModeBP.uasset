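; Game mode that manages a switchable party of Knight, Wizard and Archer characters.
; BeginPlay fills the Party class list, and SpawnPlayableCharacters spawns one member per supplied spawn location by matching index, then possesses the first.
; CycleCharacters advances through the spawned characters with wraparound, possessing the next and calling ResetControlledPawn on the PlayerControllerBP.
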(event `self.ReceiveBeginPlay`
  (`self.SetupParty`))

(event `CycleCharacters`
  (bind _returnvalue (`GameplayStatics.GetPlayerController` 0))
  ;[0 0 0] Swap between characters from the array
  (if (> (`KismetArrayLibrary.Array_Length` (`self.PlayableCharacters`)) 0)
    (bind _result (`/Engine/EditorBlueprintResources/StandardMacros.IncrementInt` (`self.CurrentPlayableCharacterIndex`))
      (:`  `
        (if (>= _result (`KismetArrayLibrary.Array_Length` (`self.PlayableCharacters`)))
          (set `self.CurrentPlayableCharacterIndex` 0))
        (`Controller.Possess` _returnvalue (`|GetArrayItem` (`self.PlayableCharacters`) (`self.CurrentPlayableCharacterIndex`)))
        (bind _asplayer_controller_bp (cast `/Game/Blueprints/PlayerControllerBP` _returnvalue))
        (`/Game/Blueprints/PlayerControllerBP.ResetControlledPawn` _asplayer_controller_bp)))))

(fn `SetupParty`
  (`KismetArrayLibrary.Array_Add` (`self.Party`) (`self.KnightSubclass`))
  (`KismetArrayLibrary.Array_Add` (`self.Party`) (`self.WizardSubclass`))
  (`KismetArrayLibrary.Array_Add` (`self.Party`) (`self.ArcherSubclass`)))

(fn `SpawnPlayableCharacters`
  (params (NewParam :type "Array of Vector Structure"))
  ;[0 0 0] Spawn playable characters into the level
  (`KismetArrayLibrary.Array_Clear` (`self.PlayableCharacters`))
  (for (_array_element _array_index) NewParam
    (bind _returnvalue (`|SpawnActorFromClass` (`|GetArrayItem` (`self.Party`) _array_index) (`KismetMathLibrary.MakeTransform` _array_element) "AdjustIfPossibleButAlwaysSpawn" "OverrideRootScale" null null))
    (`KismetArrayLibrary.Array_Add` (`self.PlayableCharacters`) _returnvalue))
  ;;[0 0 0] Possess the first character
  (`Controller.Possess` (`GameplayStatics.GetPlayerController` 0) (`|GetArrayItem` (`self.PlayableCharacters`))))

(fn `UserConstructionScript`)