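; Base projectile that damages and knocks back opposing characters, with an empty handler for friendly hits.
; Construction picks the trail from effect type or Status class and copies affiliation from the playable-character owner; BeginPlay attaches the trail as a separate persistence actor.
; Overlaps and hits share Collide, which filters out ignored objects and non-hurtbox components, then toggles Block/Overlap for bouncing.
; Non-characters always cause bounces; non-bouncing hurtbox hits consume piercing or destroy it.
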(event OnComponentBeginOverlap(Hitbox)
  (params (OverlappedComponent :type Primitive%20Component%20Object%20Reference) (OtherActor :type Actor%20Object%20Reference) (OtherComp :type Primitive%20Component%20Object%20Reference) (OtherBodyIndex :type Integer) (bFromSweep :type Boolean) (SweepResult :type Hit%20Result%20Structure%20%28by%20ref%29))
  (if (Variables|Default|GetCollisionControl)
    (CallFunction|Collide OtherActor OtherComp)
    (CallFunction|DestroySelfAttempt)))

(event EventBeginPlay
  (bind _self self)
  ;[0 0 0] Persistent Particles Setup
  (bind _returnvalue (Game|SpawnActorfromClass "/Game/Niagara/ParticlePersistenceBP.ParticlePersistenceBP_C" (Transformation|GetActorTransform) "Undefined" _self (Variables|Visuals|GetTrailEffect) _self 0))
  (bind _output_get (Variables|Components|SetTrail _returnvalue))
  (Transformation|AttachActorToActor _output_get self "None" "KeepWorld" "KeepWorld" "KeepWorld" true))

(event EventTick
  (params (DeltaSeconds :type Float%20%28single-precision%29))
  (bind _returnvalue (Transformation|GetActorLocation))
  (Transformation|SetActorRotation (Math|Rotator|FindLookatRotation _returnvalue (+ _returnvalue (Transformation|GetVelocity)))))

(event Collision|EventHit
  (params (MyComp :type Primitive%20Component%20Object%20Reference) (Other :type Actor%20Object%20Reference) (OtherComp :type Primitive%20Component%20Object%20Reference) (bSelfMoved :type Boolean) (HitLocation :type Vector :default "0, 0, 0") (HitNormal :type Vector :default "0, 0, 0") (NormalImpulse :type Vector :default "0, 0, 0") (Hit :type Hit%20Result%20Structure%20%28by%20ref%29))
  (if (Variables|Default|GetCollisionControl)
    (CallFunction|Collide Other OtherComp)
    (CallFunction|DestroySelfAttempt)))

(fn ConstructionScript
  (Transformation|SetWorldScale3D (Variables|Default|GetHitbox) "0.800000,0.800000,0.800000")
  (Utilities|FlowControl|Sequence
    (:then_0
      ;[0 0 0] Trail Effect Setup
      (switch Utilities|FlowControl|Switch|SwitchonVisualEffectTypes (Variables|Visuals|GetVisualEffectType)
        (:NewEnumerator5
          (if (Utilities|IsValidClass (Variables|Stats|GetStatus))
            (switch Utilities|FlowControl|Switch|SwitchonVisualEffectTypes (.ParticleEffectType (Utilities|GetClassDefaults (Variables|Stats|GetStatus)))
              (:NewEnumerator5
                (Variables|Visuals|SetTrailEffect "/Game/Niagara/Trail/BasicTrailSystem.BasicTrailSystem" :!label _label))
              (:NewEnumerator4
                (goto _label))
              (:NewEnumerator0
                (Variables|Visuals|SetTrailEffect "/Game/Niagara/Trail/TrailMagic.TrailMagic"))
              (:NewEnumerator1
                (Variables|Visuals|SetTrailEffect "/Game/Niagara/Trail/TrailPoison.TrailPoison"))
              (:NewEnumerator2
                (Variables|Visuals|SetTrailEffect "/Game/Niagara/Trail/TrailFire.TrailFire"))
              (:NewEnumerator3
                (Variables|Visuals|SetTrailEffect "/Game/Niagara/Trail/TrailIce.TrailIce")))
            (else
              (Variables|Visuals|SetTrailEffect "/Game/Niagara/Trail/BasicTrailSystem.BasicTrailSystem"))))
        (:NewEnumerator4
          (Variables|Visuals|SetTrailEffect "/Game/Niagara/Trail/BasicTrailSystem.BasicTrailSystem"))
        (:NewEnumerator0
          (Variables|Visuals|SetTrailEffect "/Game/Niagara/Trail/TrailMagic.TrailMagic"))
        (:NewEnumerator1
          (Variables|Visuals|SetTrailEffect "/Game/Niagara/Trail/TrailPoison.TrailPoison"))
        (:NewEnumerator2
          (Variables|Visuals|SetTrailEffect "/Game/Niagara/Trail/TrailFire.TrailFire"))
        (:NewEnumerator3
          (Variables|Visuals|SetTrailEffect "/Game/Niagara/Trail/TrailIce.TrailIce"))))
    (:then_1
      ;[0 0 0] Set Affiliation
      (bind _asplayable_character_bp (Utilities|Casting|CastToPlayableCharacterBP (Components|GetOwner)))
      (Variables|Default|SetAffiliation (Variables|/Game/Blueprints/Characters/BaseCharacterBP.BaseCharacterBP_C|GetAffiliation _asplayable_character_bp)))))

(fn HitEnemy
  (params (EnemyTarget :type Base%20Character%20BP%20Object%20Reference))
  (bind _returnvalue (Transformation|GetActorLocation EnemyTarget))
  (bind _returnvalue_2 (Components|GetOwner))
  (bind _knockback (Variables|Stats|GetKnockback))
  (bind _returnvalue_3 (Transformation|GetActorLocation _returnvalue_2))
  (bind _returnvalue_4 (Math|Vector|GetUnitDirection(Vector) _returnvalue_3 _returnvalue))
  (if (not (Variables|/Game/Blueprints/Characters/BaseCharacterBP.BaseCharacterBP_C|GetKnockedOut EnemyTarget))
    (Character|LaunchCharacter EnemyTarget (Math|Vector|MakeVector (* (* (.x _returnvalue_4) 5e+02) _knockback) (* (* (.y _returnvalue_4) 5e+02) _knockback) (* 1.5e+02 _knockback)) true true)
    (bind _result (Utilities|NegateInt (Variables|Stats|GetDamage))
      (:%20%20
        (if (!= _result 0)
          (Default|ReceiveDeltaHealth EnemyTarget _result (Components|GetOwner)))))))

(fn HitFriendly
  (params (FriendlyTarget :type Base%20Character%20BP%20Object%20Reference)))

(fn Collide
  (params (CollidedObject :type Object%20Object%20Reference) (CollidedComponent :type Primitive%20Component%20Object%20Reference))
  (bind _returnvalue (Utilities|GetClass CollidedObject))
  ;[0 0 0] Ignore certain objects
  ;;[0 0 0] Ignore owner
  (if (!= CollidedObject (Components|GetOwner))
    (if (Math|Boolean|ANDBoolean (!= _returnvalue "/Game/Blueprints/Spawnables/Pools/BasePoolBP.BasePoolBP_C") (not (Utilities|ClassIsChildOf _returnvalue "BaseProjectileBP_C")) (!= _returnvalue "/Game/Blueprints/Other/Spawners/EncounterTrigger.EncounterTrigger_C") (!= _returnvalue "/Game/Blueprints/Other/ProjectilePassableWallBP.ProjectilePassableWallBP_C"))
      ;[0 0 0] Ignore all of a character except the hurtbox
      (bind _asbase_character_bp (Utilities|Casting|CastToBaseCharacterBP CollidedObject)
        (:then
          (if (and (stale _bsuccess) (== (Variables|/Game/Blueprints/Characters/BaseCharacterBP.BaseCharacterBP_C|GetHurtbox _asbase_character_bp) CollidedComponent))
            ;[0 0 0] Whether to bounce off characters or not
            (Variables|Default|SetCorrectCollision true)
            (CallFunction|SetShouldBounce (Variables|Default|GetShouldBounceCharacters))
            ;[0 0 0] Check if a character's hurtbox of the opposite affiliation has been hit
            (if (Utilities|Enum|NotEqual(Enum) (Variables|Default|GetAffiliation) (Variables|/Game/Blueprints/Characters/BaseCharacterBP.BaseCharacterBP_C|GetAffiliation _asbase_character_bp))
              (CallFunction|HitEnemy _asbase_character_bp)
              (else
                (CallFunction|HitFriendly _asbase_character_bp)))
            (else
              ;[0 0 0] Never bounce off ignored objects (High Priority)
              (Variables|Default|SetCorrectCollision false :!label _label)
              (CallFunction|SetShouldBounce false))))
        (:CastFailed
          ;[0 0 0] Always bounce off non characters (Low Priority)
          (Variables|Default|SetCorrectCollision true)
          (CallFunction|SetShouldBounce true)))
      (else
        (goto _label)))
    (else
      (goto _label))))

(fn DestroySelfAttempt
  (if (and (Variables|Default|GetCorrectCollision) (not (Variables|Default|GetShouldBounce)))
    (if (not (Variables|Stats|Piercing|GetPiercing))
      (Actor|DestroyActor :!label _label)
      (else
        ;[0 0 0] Can pierce targets equal to PiercingPower
        (if (> (Variables|Stats|Piercing|GetPiercingPower) 0)
          (Math|Integer|DecrementInt (Variables|Stats|Piercing|GetPiercingPower))
          (else
            (goto _label)))))))

(fn SetShouldBounce
  (params (ShouldBounce :type Boolean))
  (LocalVariables|SetCollisionControlSave (Variables|Default|GetCollisionControl))
  (Variables|Default|SetCollisionControl false)
  (bind _output_get (Variables|Default|SetShouldBounce ShouldBounce))
  (if _output_get
    (Collision|SetCollisionResponsetoChannel (Variables|Default|GetHitbox) "ECC_WorldDynamic" "ECR_Block")
    (else
      (Collision|SetCollisionResponsetoChannel (Variables|Default|GetHitbox) "ECC_WorldDynamic" "ECR_Overlap")))
  (Variables|Default|SetCollisionControl (LocalVariables|GetCollisionControlSave)))