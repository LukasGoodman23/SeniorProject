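; Area-of-effect spell projectile that leaves a status pool where it lands on flat, static ground.
; Construction tints a dynamic spell material and picks a trail from the status effect class.
; Hit flags near-level surfaces by normal angle, then Collide stops bouncing and spawns BasePoolBP with the status, lifespan and owner's affiliation.
; Character bouncing turns on only after leaving the owner's hurtbox, avoiding initial self-interaction.
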(event `self.Hitbox.OnComponentBeginOverlap`
  (params (OverlappedComponent :type "PrimitiveComponent Object Reference") (OtherActor :type "Actor Object Reference") (OtherComp :type "PrimitiveComponent Object Reference") (OtherBodyIndex :type Integer) (bFromSweep :type Boolean) (SweepResult :type "HitResult Structure (by ref)"))
  (set `self.HitFlatSurface` false))

(event `self.ReceiveHit`
  (params (MyComp :type "PrimitiveComponent Object Reference") (Other :type "Actor Object Reference") (OtherComp :type "PrimitiveComponent Object Reference") (bSelfMoved :type Boolean) (HitLocation :type "Vector Structure") (HitNormal :type "Vector Structure") (NormalImpulse :type "Vector Structure") (Hit :type "HitResult Structure (by ref)"))
  ;[0 0 0] Only collide if on a flat surface
  (set `self.HitFlatSurface` (<= (`KismetMathLibrary.DegAcos` (`KismetMathLibrary.Dot_VectorVector` HitNormal (0.0 0.0 1.0))) 15.0))
  (set `self.Hit Location` HitLocation)
  (`parent.ReceiveHit` null Other OtherComp false (0.0 0.0 0.0) (0.0 0.0 0.0) (0.0 0.0 0.0) Hit))

(event `self.Hitbox.OnComponentEndOverlap`
  (params (OverlappedComponent :type "PrimitiveComponent Object Reference") (OtherActor :type "Actor Object Reference") (OtherComp :type "PrimitiveComponent Object Reference") (OtherBodyIndex :type Integer))
  ;[0 0 0] Makes sure the projectile does not initially interact with the owner
  (if (== OtherActor (`self.GetOwner`))
    (bind _asbase_character_bp (cast `/Game/Blueprints/Characters/BaseCharacterBP` OtherActor))
    (if (== (`/Game/Blueprints/Characters/BaseCharacterBP.Hurtbox` _asbase_character_bp) OtherComp)
      (set `self.ShouldBounceCharacters` true))))

(fn `Collide`
  (params (CollidedObject :type "Object Object Reference") (CollidedComponent :type "PrimitiveComponent Object Reference"))
  (bind _returnvalue (`self.GetOwner`))
  (bind (_returnvalue_location _returnvalue_rotation) (`KismetMathLibrary.BreakTransform` (`self.GetTransform` self)))
  (`parent.Collide` CollidedObject CollidedComponent)
  ;[0 0 0] Hit a flat, static object
  (if (and (`self.CorrectCollision`) (`self.HitFlatSurface`) (`|EnumEquality` (`PrimitiveComponent.GetCollisionObjectType` CollidedComponent) "ECC_WorldStatic"))
    (set `self.CollisionControl` false)
    (`self.SetShouldBounce` false)
    ;[0 0 0] Spawn pool
    (`|SpawnActorFromClass` "/Game/Blueprints/Spawnables/Pools/BasePoolBP.BasePoolBP_C" (`KismetMathLibrary.MakeTransform` (`self.Hit Location`) _returnvalue_rotation) "Undefined" "OverrideRootScale" _returnvalue (`self.Status`) (`self.PoolLifespan`) (`/Game/Blueprints/Characters/BaseCharacterBP.Affiliation` (cast `/Game/Blueprints/Characters/BaseCharacterBP` _returnvalue :!pure true)) null)))

(fn `UserConstructionScript`
  (locals (Color :type "LinearColor Structure" :default (struct :`G` 0.759054 :`B` 1.0 :`A` 1.0)))
  (`parent.UserConstructionScript`)
  ;[0 0 0] Visual setup
  (bind _returnvalue (`PrimitiveComponent.CreateDynamicMaterialInstance` (`self.Mesh`) 0 "/Game/Materials/MagicSpell.MagicSpell" "None"))
  (if (`KismetSystemLibrary.IsValidClass` (`self.Status`))
    (`|ExecutionSequence`
      (:`then_0`
        (switch `/Game/Blueprints/StatusComponents/StatusEffect` (`.StatusEffect` (defaults `Object` (`self.Status`)))
          (:`NewEnumerator0`
            (set `local.Color` (struct :`B` 1.0 :`A` 1.0))
            (set `self.TrailEffect` "/Game/Niagara/Trail/TrailMagic.TrailMagic"))
          (:`NewEnumerator1`
            (set `local.Color` (struct :`G` 1.0 :`A` 1.0))
            (set `self.TrailEffect` "/Game/Niagara/Trail/TrailPoison.TrailPoison"))
          (:`NewEnumerator2`
            (set `local.Color` (struct :`R` 1.0 :`G` 0.25 :`A` 1.0)))
          (:`NewEnumerator3`
            (set `local.Color` (struct :`G` 1.0 :`B` 1.0 :`A` 1.0)))))
      (:`then_1`
        (`MaterialInstanceDynamic.SetVectorParameterValue` _returnvalue "Color" (`local.Color`))))))