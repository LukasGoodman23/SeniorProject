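; Contact projectile Blueprint that can inflict a status effect on the enemies it hits, extending a parent projectile class.
; On an enemy hit it runs the parent logic, then, if a Status class is set, adds it to the target as a component with its lifetime set from StatusDuration.
; On a friendly hit it runs the parent logic, then clears the CorrectCollision flag.
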(fn `HitEnemy`
  (params (EnemyTarget :type "/Game/Blueprints/Characters/BaseCharacterBP Object Reference"))
  (bind _status (`self.Status`))
  (`parent.HitEnemy` EnemyTarget)
  ;[0 0 0] Inflict status if any
  (if (`KismetSystemLibrary.IsValidClass` _status)
    (`|AddComponentByClass` EnemyTarget _status (`self.StatusDuration`))))

(fn `HitFriendly`
  (params (FriendlyTarget :type "/Game/Blueprints/Characters/BaseCharacterBP Object Reference"))
  (`parent.HitFriendly` FriendlyTarget)
  (set `self.CorrectCollision` false))

(fn `UserConstructionScript`
  (`parent.UserConstructionScript`))