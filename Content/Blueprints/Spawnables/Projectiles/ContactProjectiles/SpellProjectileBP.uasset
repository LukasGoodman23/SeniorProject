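; Spell projectile whose color and trail reflect the status effect class it carries.
; The construction script puts a dynamic MagicSpell material on the mesh, then reads the Status class default to choose a color and trail for Regen, Poison, Burn or Ice.
; The color feeds the material's Color parameter and the trail is stored in TrailEffect.
; The event graph adds no logic of its own.
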(fn `UserConstructionScript`
  (locals (Color :type "LinearColor Structure"))
  (`parent.UserConstructionScript`)
  ;[0 0 0] Visual setup
  (bind _returnvalue (`PrimitiveComponent.CreateDynamicMaterialInstance` (`self.Mesh`) 0 "/Game/Materials/MagicSpell.MagicSpell" "None"))
  (if (`KismetSystemLibrary.IsValidClass` (`self.Status`))
    (`|ExecutionSequence`
      (:`then_0`
        (switch `/Game/Blueprints/StatusComponents/StatusEffect` (`.StatusEffect` (defaults `Object` (`self.Status`)))
          (:`NewEnumerator0`
            (set `local.Color` (struct :`B` 1.0 :`A` 1.0))
            (set `self.TrailEffect` "/Game/Niagara/Trail/TrailMagic.TrailMagic"))
          (:`NewEnumerator1`
            (set `local.Color` (struct :`G` 1.0 :`A` 1.0))
            (set `self.TrailEffect` "/Game/Niagara/Trail/TrailPoison.TrailPoison"))
          (:`NewEnumerator2`
            (set `local.Color` (struct :`R` 1.0 :`G` 0.25 :`A` 1.0))
            (set `self.TrailEffect` "/Game/Niagara/Trail/TrailFireRibbon_System.TrailFireRibbon_System"))
          (:`NewEnumerator3`
            (set `local.Color` (struct :`G` 1.0 :`B` 1.0 :`A` 1.0))
            (set `self.TrailEffect` "/Game/Niagara/Trail/TrailIce.TrailIce"))))
      (:`then_1`
        (`MaterialInstanceDynamic.SetVectorParameterValue` _returnvalue "Color" (`local.Color`))))))