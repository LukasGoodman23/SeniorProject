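; Base actor for timed status-effect pools that apply their StatusEffect component to living characters inside, choosing allies or opponents from the effect's class defaults.
; Overlap begin and a per-tick check both attempt application, catching cases like revives inside the pool.
; The construction script previews Niagara particles by effect type; at runtime a ParticlePersistenceBP replaces them, with affiliation-colored outlines and area-scaled spawning.
; Regen pools register themselves as HealingPool in playable characters' blackboards.
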(event `self.ReceiveBeginPlay`
  (bind _particles (`self.Particles`))
  ;[0 0 0] Persistent Particles Setup
  (`ActorComponent.Deactivate` (`self.Particles`))
  (bind _returnvalue (`|SpawnActorFromClass` "/Game/Niagara/ParticlePersistenceBP.ParticlePersistenceBP_C" (`SceneComponent.K2_GetComponentToWorld` _particles) "Undefined" "OverrideRootScale" self (`NiagaraComponent.GetAsset` _particles) self null))
  (bind _output_get (set `self.Trail` _returnvalue))
  (`self.K2_AttachToActor` _output_get self "None" "KeepWorld" "KeepWorld" "KeepWorld" true)
  (`self.SetupParticleSystem` (`/Game/Niagara/ParticlePersistenceBP.Emitter` (`self.Trail`)))
  (`self.SetLifeSpan` (`self.Lifespan`))
  (if (== (`self.StatusEffect`) "/Game/Blueprints/StatusComponents/StatusTypes/IntervalStatuses/DamageOverTime/RegenBP.RegenBP_C")
    (bind _outactors (`GameplayStatics.GetAllActorsOfClass` "/Game/Blueprints/Characters/PlayableCharacters/PlayableCharacterBP.PlayableCharacterBP_C"))
    (for _array_element _outactors
      (bind _returnvalue_2 (`AIBlueprintHelperLibrary.GetBlackboard` _array_element))
      (`/Engine/EditorBlueprintResources/StandardMacros.IsValid` _returnvalue_2
        (:`Is Valid`
          (`BlackboardComponent.SetValueAsObject` _returnvalue_2 "HealingPool" self))))))

(event `self.ReceiveTick`
  (params (DeltaSeconds :type "Float (single-precision)"))
  ;[0 0 0] Constantly knows what is in it (accounts for situations where a character revives inside of the pool, for example)
  (for _array_element (`self.GetOverlappingActors` "/Game/Blueprints/Characters/BaseCharacterBP.BaseCharacterBP_C")
    (bind _asbase_character_bp (cast `/Game/Blueprints/Characters/BaseCharacterBP` _array_element))
    (`self.AttemptApplyStatus` _asbase_character_bp)))

(event `self.Hitbox.OnComponentBeginOverlap`
  (params (OverlappedComponent :type "PrimitiveComponent Object Reference") (OtherActor :type "Actor Object Reference") (OtherComp :type "PrimitiveComponent Object Reference") (OtherBodyIndex :type Integer) (bFromSweep :type Boolean) (SweepResult :type "HitResult Structure (by ref)"))
  (bind _asbase_character_bp (cast `/Game/Blueprints/Characters/BaseCharacterBP` OtherActor))
  (`self.AttemptApplyStatus` _asbase_character_bp))

(fn `AttemptApplyStatus`
  (params (Character :type "/Game/Blueprints/Characters/BaseCharacterBP Object Reference"))
  (if (`PrimitiveComponent.IsOverlappingComponent` (`/Game/Blueprints/Characters/BaseCharacterBP.Hurtbox` Character) (`self.Hitbox`))
    (if (not (`/Game/Blueprints/Characters/BaseCharacterBP.KnockedOut` Character))
      (if true
        (if (defaults `Object` (`self.StatusEffect`))
          (if (`|EnumInequality` (`self.Affiliation`) (`/Game/Blueprints/Characters/BaseCharacterBP.Affiliation` Character))
            (`|AddComponentByClass` Character (`self.StatusEffect`) 0.0 :!label _label))
          (elif (`|EnumEquality` (`self.Affiliation`) (`/Game/Blueprints/Characters/BaseCharacterBP.Affiliation` Character))
            (goto _label)))))))

(fn `SetupParticleSystem`
  (params (NiagaraComponent :type "NiagaraComponent Object Reference"))
  (locals (System :type "NiagaraComponent Object Reference"))
  (bind (_returnvalue_x _returnvalue_y) (`KismetMathLibrary.BreakVector` (`SceneComponent.K2_GetComponentScale` (`self.Hitbox`))))
  (set `local.System` NiagaraComponent)
  (`|ExecutionSequence`
    (:`then_0`
      ;[0 0 0] Set the color of the outline according to the pool's affiliation
      (switch `/Game/Blueprints/Characters/Affiliation` (`self.Affiliation`)
        (:`NewEnumerator0`
          (`NiagaraComponent.SetVariableMaterial` (`local.System`) "OutlineMaterial" "/Game/Materials/SolidColors/BlueWizard.BlueWizard"))
        (:`NewEnumerator1`
          (`NiagaraComponent.SetVariableMaterial` (`local.System`) "OutlineMaterial" "/Game/Materials/SolidColors/RedKnight.RedKnight"))))
    (:`then_1`
      ;[0 0 0] Adjusts the spawn rate using a custom multiplier and the area of the pool
      (`NiagaraComponent.SetNiagaraVariableFloat` (`local.System`) "SurfaceArea" (`KismetMathLibrary.MultiplyByPi` (* (* _returnvalue_x 50.0) (* _returnvalue_y 50.0))))
      (`NiagaraComponent.SetNiagaraVariableFloat` (`local.System`) "SpawnRate" (`self.ParticleSpawnRate`)))))

(fn `UserConstructionScript`
  (bind _particles (`self.Particles`))
  ;[0 0 0] Particle Setup (For Preview)
  (`|ExecutionSequence`
    (:`then_0`
      (switch `/Game/Niagara/VisualEffectTypes` (`.ParticleEffectType` (defaults `Object` (`self.StatusEffect`)))
        (:`NewEnumerator0`
          (`NiagaraComponent.SetAsset` _particles "/Game/Niagara/StatusArea/AreaRegen.AreaRegen" true))
        (:`NewEnumerator1`
          (`NiagaraComponent.SetAsset` _particles "/Game/Niagara/StatusArea/AreaPoison.AreaPoison" true))
        (:`NewEnumerator2`
          (`NiagaraComponent.SetAsset` _particles "/Game/Niagara/StatusArea/AreaBurn.AreaBurn" true))
        (:`NewEnumerator3`
          (`NiagaraComponent.SetAsset` _particles "/Game/Niagara/StatusArea/AreaSlow.AreaSlow" true))))
    (:`then_1`
      (`self.SetupParticleSystem` (`self.Particles`)))))