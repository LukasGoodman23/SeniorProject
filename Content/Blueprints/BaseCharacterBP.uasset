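; Base character Blueprint that provides health, damage and knockout handling.
; ApplyDamage negates a positive amount and passes it to the target's ReceiveHealthChange, which heals or damages.
; At zero or below, health is set to zero and the character is knocked out, ignoring further health changes.
; A debug key runs a capsule trace at the actor's location, damages BaseCharacterBP hits and prints their health.
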(event `ReceiveHealthChange`
  (params (HealthAdded :type Integer))
  ;[0 0 0] Receive a change in Health (positive HealthAdded heals, negative Health Added damages)
  ; Cannot recieve a Health change if knocked out, becomes knocked out if Health becomes negative or zero
  ; If Health is negative when knocked out, it is set to zero.
  (if (not (`self.IsKnockedOut`))
    (bind _output_get (set `self.Health` (+ HealthAdded (`self.Health`))))
    (if (<= _output_get 0)
      (set `self.IsKnockedOut` true)
      (set `self.Health` 0))))

(event `self.ReceiveTick`
  (params (DeltaSeconds :type "Float (single-precision)")))

(event `ApplyDamage`
  (params (TargetReceiver :type "/Game/Blueprints/BaseCharacterBP Object Reference") (DamageDealt :type Integer))
  ;[0 0 0] Apply damage to another BaseCharacterBP (TargetReceiver)
  ; DamageDealth should be positive and will be negated when applying damage
  (`self.ReceiveHealthChange` TargetReceiver (* DamageDealt -1)))

(event `InputAction|DEBUG_KEY1`
  (params (Key :type "Key Structure"))
  (bind _returnvalue (`self.K2_GetActorLocation`))
  ;[0.4667 0.2678 0] DEBUG (Num Pad 1): Checks nearby collision for nearby characters and does damage to them
  ; Tests ApplyDamage and ReceiveHealthChange custom events
  (:`Pressed`
    (bind _outhits (`KismetSystemLibrary.CapsuleTraceMulti` :`Start` _returnvalue :`End` _returnvalue :`Radius` 70.0 :`HalfHeight` 70.0 :`TraceChannel` "TraceTypeQuery1" :`DrawTime` 2.0))
    (for _array_element _outhits
      (bind _asbase_character_bp (cast `/Game/Blueprints/BaseCharacterBP` (`.HitActor` (`GameplayStatics.BreakHitResult` _array_element))))
      (`self.ApplyDamage` _asbase_character_bp 10)
      (`KismetSystemLibrary.PrintString` (`KismetStringLibrary.Conv_IntToString` (`/Game/Blueprints/BaseCharacterBP.Health` _asbase_character_bp))))))

(fn `UserConstructionScript`)