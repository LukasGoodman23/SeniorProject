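; Playable Wizard character class with two spell actions: a forward-moving projectile and a lobbed spell that creates a pool effect.
; Each action is gated by ready, busy and knocked-out checks, then plays a reused Knight attack animation between rotation begin and end calls.
; Start and end lag delays time the projectile spawn, which receives damage, knockback, status and visual effect settings.
; The construction script attaches the weapon mesh to the right-hand socket.
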(event `self.Action1`
  ;[0 0 0] Preparation
  (if (and (`self.Action1Ready`) (not (`self.PerformingAction`)) (not (`self.KnockedOut`)))
    (set `self.PerformingAction` true)
    (set `self.Action1Ready` false)
    (`self.RotateForActionBegin`)
    (`SkeletalMeshComponent.PlayAnimation` (`self.Mesh`) "/Game/Characters/Heroes/anims/anim-knight/KnightAttkLight.KnightAttkLight" false)
    (`KismetSystemLibrary.Delay` (`self.Action1StartLag`))
    ;[0 0 0] Fire Forward-Moving Spell (To contact a character)
    (`|SpawnActorFromClass` (`self.Action1ProjectileClass`) (`SceneComponent.K2_GetComponentToWorld` (`self.CapsuleComponent`)) "Undefined" "OverrideRootScale" self 5.0 false 1 (`self.Action1Damage`) (`self.Action1Knockback`) (`self.Action1ProjectileStatus`) (`self.Action1VisualEffectType`) self)
    (`KismetSystemLibrary.Delay` (`self.Action1EndLag`))
    ;[0 0 0] End/Cleanup
    (`SkeletalMeshComponent.SetAnimationMode` (`self.Mesh`) "AnimationBlueprint")
    (`self.RotateForActionEnd`)
    (set `self.PerformingAction` false)))

(event `self.Action2`
  ;[0 0 0] Preparation
  (if (and (`self.Action2Ready`) (not (`self.PerformingAction`)) (not (`self.KnockedOut`)))
    (set `self.PerformingAction` true)
    (set `self.Action2Ready` false)
    (`self.RotateForActionBegin`)
    (`SkeletalMeshComponent.PlayAnimation` (`self.Mesh`) "/Game/Characters/Heroes/anims/anim-knight/KnightAttkHeavy.KnightAttkHeavy" false)
    (`KismetSystemLibrary.Delay` (`self.Action2StartLag`))
    ;[0 0 0] Lob a Pool Effect Spell
    (`|SpawnActorFromClass` (`self.Action2ProjectileClass`) (`SceneComponent.K2_GetComponentToWorld` (`self.CapsuleComponent`)) "Undefined" "OverrideRootScale" self (`self.LobPoolLifespan`) false 1 (`self.Action2Damage`) (`self.Action2Knockback`) (`self.LobPoolEffect`) (`self.Action2VisualEffectType`) self)
    (`KismetSystemLibrary.Delay` (`self.Action2EndLag`))
    ;[0 0 0] End/Cleanup
    (`SkeletalMeshComponent.SetAnimationMode` (`self.Mesh`) "AnimationBlueprint")
    (`self.RotateForActionEnd`)
    (set `self.PerformingAction` false)))

(fn `UserConstructionScript`
  (`parent.UserConstructionScript`)
  (`SceneComponent.K2_AttachToComponent` (`self.WeaponPrimaryMesh`) (`self.Mesh`) "RightHand" "KeepRelative" "KeepRelative" "KeepRelative" true))