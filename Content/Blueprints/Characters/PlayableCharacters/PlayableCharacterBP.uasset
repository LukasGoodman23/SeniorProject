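; Base Blueprint for a playable character that handles camera-relative movement and getting knocked out.
; MoveForward and MoveRight add movement input along control-yaw directions, ignored once the character is knocked out.
; KnockOut fires once, reporting it and triggering KnockOutSwap, which increments the game mode's knockout count.
; After a short delay, a player-controlled character has the game mode check for game over and otherwise cycle to another character.
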(event `KnockOutSwap`
  (bind _asmain_game_mode_bp (cast `/Game/Blueprints/MainGameModeBP` (`GameplayStatics.GetGameMode`) :!pure true))
  (bind _asplayer_controller_bp (cast `/Game/Blueprints/PlayerControllerBP` (`self.GetController`) :!pure true))
  ;[0 0 0] Occurs upon knock out: Forces a swap after a delay if needed
  (`/Engine/EditorBlueprintResources/StandardMacros.IncrementInt` (`/Game/Blueprints/MainGameModeBP.KnockedOutCharacters` _asmain_game_mode_bp)
    (:`  `
      (`KismetSystemLibrary.Delay` 2.0)
      (`/Engine/EditorBlueprintResources/StandardMacros.IsValid` _asplayer_controller_bp
        (:`Is Valid`
          (bind _gameover (`/Game/Blueprints/MainGameModeBP.CheckForGameOver` _asmain_game_mode_bp))
          (if (not _gameover)
            (`/Game/Blueprints/MainGameModeBP.Cycle Character` _asmain_game_mode_bp _asplayer_controller_bp)))))))

(fn `KnockOut`
  (if (not (`self.KnockedOut`))
    (set `self.KnockedOut` true)
    (`KismetSystemLibrary.PrintString` (`KismetStringLibrary.Concat_StrStr` (`KismetSystemLibrary.GetDisplayName` self) " is knocked out!"))
    (`self.KnockOutSwap`)))

(fn `MoveForward`
  (params (ScaleValue :type "Float (double-precision)"))
  (if (not (`self.KnockedOut`))
    (`self.AddMovementInput` (`KismetMathLibrary.GetForwardVector` (`KismetMathLibrary.MakeRotator` 0.0 0.0 (.yaw (`self.GetControlRotation`)))) ScaleValue)))

(fn `MoveRight`
  (params (ScaleValue :type "Float (double-precision)"))
  (if (not (`self.KnockedOut`))
    (`self.AddMovementInput` (`KismetMathLibrary.GetRightVector` (`KismetMathLibrary.MakeRotator` 0.0 0.0 (.yaw (`self.GetControlRotation`)))) ScaleValue)))

(fn `UserConstructionScript`
  (`parent.UserConstructionScript`))