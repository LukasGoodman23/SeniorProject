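; Character component that tracks nearby characters and lets its owner interact with them, currently to manually revive knocked-out ones.
; A query-only sphere created at BeginPlay maintains the interactable list through overlap events, filtered by hurtbox overlap and excluding the owner.
; Interact starts reviving the first knocked-out entry via its KnockoutStatusBP, and StopInteracting cancels, also when that target leaves range.
; Tick and range exit toggle revival meter widgets according to possession.
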(event `self.ReceiveBeginPlay`
  (set `self.Owner` (cast `/Game/Blueprints/Characters/BaseCharacterBP` (`self.GetOwner`) :!pure true))
  ;[0 0 0] Get characters in range on spawn
  (`self.CreateRangeOverlap` (delegate `BeginOverlap`) (delegate `EndOverlap`))
  (for _array_element (`PrimitiveComponent.GetOverlappingComponents` (`self.InteractionArea`))
    (if (`self.ComponentHasTag` _array_element "Hurtbox")
      (`self.AddInteractable` (`self.GetOwner` _array_element)))))

(event `BeginOverlap`
  (params (OverlappedComponent :type "PrimitiveComponent Object Reference") (OtherActor :type "Actor Object Reference") (OtherComp :type "PrimitiveComponent Object Reference") (OtherBodyIndex :type Integer) (bFromSweep :type Boolean) (SweepResult :type "HitResult Structure (by ref)"))
  (`self.AddInteractable` OtherActor))

(event `EndOverlap`
  (params (OverlappedComponent :type "PrimitiveComponent Object Reference") (OtherActor :type "Actor Object Reference") (OtherComp :type "PrimitiveComponent Object Reference") (OtherBodyIndex :type Integer))
  (`self.RemoveInteractable` OtherActor))

(event `self.ReceiveTick`
  (params (DeltaSeconds :type "Float (single-precision)"))
  (for _array_element (`self.InteractableCharacters`)
    (`|ExecutionSequence`
      (:`then_0`
        (if (`/Game/Blueprints/Characters/BaseCharacterBP.KnockedOut` _array_element)
          (bind _asplayable_character_bp (cast `/Game/Blueprints/Characters/PlayableCharacters/PlayableCharacterBP` (`self.Owner`)))
          (if (`/Game/Blueprints/Characters/PlayableCharacters/PlayableCharacterBP.Possessed` _asplayable_character_bp)
            (bind _revivalmeterwidget (`/Game/Blueprints/StatusComponents/StatusTypes/KnockoutStatusBP.RevivalMeterWidget` (`Actor.GetComponentByClass` _array_element "/Game/Blueprints/StatusComponents/StatusTypes/KnockoutStatusBP.KnockoutStatusBP_C")))
            (`Widget.SetVisibility` _revivalmeterwidget "Visible")
            (break)
            (elif (not (`KismetArrayLibrary.Array_Contains` (`/Game/Blueprints/Characters/Interaction.InteractableCharacters` (`/Game/Blueprints/Characters/BaseCharacterBP.Interaction` (cast `/Game/Blueprints/Characters/BaseCharacterBP` (`/Game/Blueprints/PlayerControllerBP.ControlledCharacter` (cast `/Game/Blueprints/PlayerControllerBP` (`GameplayStatics.GetPlayerController` 0) :!pure true)) :!pure true))) _array_element))
              (`Widget.SetVisibility` _revivalmeterwidget "Hidden")
              (break)
              (else
                (break)))))))))

(fn `AddInteractable`
  (params (CharacterInRange :type "Actor Object Reference"))
  (locals (NewInteractableCharacter :type "/Game/Blueprints/Characters/BaseCharacterBP Object Reference"))
  (bind _asbase_character_bp (cast `/Game/Blueprints/Characters/BaseCharacterBP` CharacterInRange))
  (bind _output_get (set `local.NewInteractableCharacter` _asbase_character_bp))
  ;[0 0 0] Makes sure the hurtbox is encountered (and prevents self)
  (if (and (`PrimitiveComponent.IsOverlappingComponent` (`self.InteractionArea`) (`/Game/Blueprints/Characters/BaseCharacterBP.Hurtbox` _output_get)) (!= (`self.Owner`) (`local.NewInteractableCharacter`)))
    (`KismetArrayLibrary.Array_AddUnique` (`self.InteractableCharacters`) (`local.NewInteractableCharacter`))))

(fn `CreateRangeOverlap`
  (params (BeginOverlap :type "Delegate (by ref)") (EndOverlap :type "Delegate (by ref)"))
  (bind _returnvalue (`|AddComponentByClass` (`self.GetOwner`) "/Script/Engine.SphereComponent" false (`KismetMathLibrary.MakeTransform` (0.0 0.0 0.0))))
  (bind _output_get (set `self.InteractionArea` _returnvalue))
  (`PrimitiveComponent.SetCollisionEnabled` _output_get "QueryOnly")
  (`PrimitiveComponent.SetCollisionObjectType` _output_get "ECC_WorldStatic")
  (`SceneComponent.SetHiddenInGame` _output_get true false)
  (`SphereComponent.SetSphereRadius` _output_get (`self.InteractionRange`) true)
  (add `PrimitiveComponent.OnComponentBeginOverlap` _output_get BeginOverlap)
  (add `PrimitiveComponent.OnComponentEndOverlap` _output_get EndOverlap))

(fn `Interact`
  (locals (InteractAttempt :type "/Game/Blueprints/Characters/BaseCharacterBP Object Reference"))
  (bind _interactattempt (`local.InteractAttempt`))
  (if (not (`/Game/Blueprints/Characters/BaseCharacterBP.KnockedOut` (`self.Owner`)))
    (for _array_element (`self.InteractableCharacters`)
      (bind _output_get (set `local.InteractAttempt` _array_element))
      ;[0 0 0] Interact with first item
      ; (Queue-Based)
      (`/Engine/EditorBlueprintResources/StandardMacros.IsValid` _output_get
        (:`Is Valid`
          ;[0 0 0] Run through possible actions
          (`|ExecutionSequence`
            (:`then_0`
              ;[0 0 0] Revive
              (if (`/Game/Blueprints/Characters/BaseCharacterBP.KnockedOut` _interactattempt)
                (set `/Game/Blueprints/StatusComponents/StatusTypes/KnockoutStatusBP.ManualReviving` true (`Actor.GetComponentByClass` _interactattempt "/Game/Blueprints/StatusComponents/StatusTypes/KnockoutStatusBP.KnockoutStatusBP_C"))
                (set `self.InteractingWith` (`local.InteractAttempt`))
                (break)))))
        (:`Is Not Valid`
          (`KismetSystemLibrary.PrintString` "ERROR (Interaction): A Non-Character shouldn't be interactable."))))))

(fn `RemoveInteractable`
  (params (CharacterInRange :type "Actor Object Reference"))
  (locals (OldInteractableCharacter :type "/Game/Blueprints/Characters/BaseCharacterBP Object Reference"))
  (bind _oldinteractablecharacter (`local.OldInteractableCharacter`))
  (bind _asbase_character_bp (cast `/Game/Blueprints/Characters/BaseCharacterBP` CharacterInRange))
  (bind _output_get (set `local.OldInteractableCharacter` _asbase_character_bp))
  ;[0 0 0] Make sure the hurtbox is what left
  (if (not (`PrimitiveComponent.IsOverlappingComponent` (`/Game/Blueprints/Characters/BaseCharacterBP.Hurtbox` _output_get) (`self.InteractionArea`)))
    ;[0 0 0] Cancel interaction if necessary
    (if (== (`self.InteractingWith`) (`local.OldInteractableCharacter`))
      (`self.StopInteracting`))
    (`KismetArrayLibrary.Array_RemoveItem` (`self.InteractableCharacters`) (`local.OldInteractableCharacter`))
    ;[0 0 0] Turn off appropriate widgets
    (bind _asplayable_character_bp (cast `/Game/Blueprints/Characters/PlayableCharacters/PlayableCharacterBP` (`self.Owner`)))
    (if (`/Game/Blueprints/Characters/PlayableCharacters/PlayableCharacterBP.Possessed` _asplayable_character_bp)
      (`|ExecutionSequence`
        (:`then_0`
          (if (`/Game/Blueprints/Characters/BaseCharacterBP.KnockedOut` _oldinteractablecharacter)
            (`Widget.SetVisibility` (`/Game/Blueprints/StatusComponents/StatusTypes/KnockoutStatusBP.RevivalMeterWidget` (`Actor.GetComponentByClass` _oldinteractablecharacter "/Game/Blueprints/StatusComponents/StatusTypes/KnockoutStatusBP.KnockoutStatusBP_C")) "Hidden")))))))

(fn `StopInteracting`
  (bind _interactingwith (`self.InteractingWith`))
  (`/Engine/EditorBlueprintResources/StandardMacros.IsValid` (`self.InteractingWith`)
    (:`Is Valid`
      (`|ExecutionSequence`
        (:`then_0`
          ;[0 0 0] Stop Reviving
          (if (`/Game/Blueprints/Characters/BaseCharacterBP.KnockedOut` _interactingwith)
            (set `/Game/Blueprints/StatusComponents/StatusTypes/KnockoutStatusBP.ManualReviving` false (`Actor.GetComponentByClass` _interactingwith "/Game/Blueprints/StatusComponents/StatusTypes/KnockoutStatusBP.KnockoutStatusBP_C"))))
        (:`then_1`
          (set `self.InteractingWith` null))))))