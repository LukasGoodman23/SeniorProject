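; Archer enemy class with a ranged attack and a melee attack, both gated by ready flags and a shared busy flag.
; Action1 plays an attack animation and spawns a projectile from the capsule transform after a start lag.
; Action2 reveals the right-hand secondary weapon and opens a timed hitbox that damages and knocks back each opposing-affiliation character once per swing.
; The construction script attaches both weapons and the hitbox.
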(event `self.Action1`
  ;[0 0 0] Preparation
  (if (and (`self.Action1Ready`) (not (`self.PerformingAction`)))
    (set `self.PerformingAction` true)
    (set `self.Action1Ready` false)
    (`SkeletalMeshComponent.PlayAnimation` (`self.Mesh`) "/Game/Characters/Heroes/anims/anim-ranger/RangerAttk.RangerAttk" false)
    (`KismetSystemLibrary.Delay` (`self.Action1StartLag`))
    ;[0 0 0] Fire Arrow
    (`|SpawnActorFromClass` "/Game/Blueprints/Spawnables/Projectiles/ContactProjectileBP.ContactProjectileBP_C" (`SceneComponent.K2_GetComponentToWorld` (`self.CapsuleComponent`)) "Undefined" "OverrideRootScale" self null 5.0 false 0 (`self.Action1Damage`) (`self.Action1Knockback`) self)
    (`KismetSystemLibrary.Delay` (`self.Action1EndLag`))
    ;[0 0 0] End/Cleanup
    (`SkeletalMeshComponent.SetAnimationMode` (`self.Mesh`) "AnimationBlueprint")
    (set `self.PerformingAction` false)))

(event `self.Action2`
  ;[0 0 0] Preparation
  (if (and (`self.Action2Ready`) (not (`self.PerformingAction`)))
    (set `self.PerformingAction` true)
    (set `self.Action2Ready` false)
    (`SkeletalMeshComponent.PlayAnimation` (`self.Mesh`) "/Game/Characters/Heroes/anims/anim-knight/KnightAttkLight.KnightAttkLight" false)
    (`SceneComponent.SetHiddenInGame` (`self.WeaponSecondaryMesh`) false false)
    (`KismetSystemLibrary.RetriggerableDelay` (`self.Action2StartLag`))
    ;[0 0 0] Active Hitbox
    (`PrimitiveComponent.SetCollisionEnabled` (`self.AttackCollision`) "QueryOnly")
    (`KismetSystemLibrary.RetriggerableDelay` (- (`self.Action2Duration`) (+ (`self.Action2StartLag`) (`self.Action2EndLag`))))
    (`PrimitiveComponent.SetCollisionEnabled` (`self.AttackCollision`) "NoCollision")
    (`KismetSystemLibrary.RetriggerableDelay` (`self.Action2EndLag`))
    ;[0 0 0] End/Cleanup
    (`SkeletalMeshComponent.SetAnimationMode` (`self.Mesh`) "AnimationBlueprint")
    (`SceneComponent.SetHiddenInGame` (`self.WeaponSecondaryMesh`) true false)
    (set `self.PerformingAction` false)
    (`KismetArrayLibrary.Array_Clear` (`self.HitCharacters`))))

(event `self.AttackCollision.OnComponentBeginOverlap`
  (params (OverlappedComponent :type "PrimitiveComponent Object Reference") (OtherActor :type "Actor Object Reference") (OtherComp :type "PrimitiveComponent Object Reference") (OtherBodyIndex :type Integer) (bFromSweep :type Boolean) (SweepResult :type "HitResult Structure (by ref)"))
  (bind _action2knockback (`self.Action2Knockback`))
  ;[0 0 0] Melee Hit
  (if (!= OtherActor self)
    (bind _asbase_character_bp (cast `/Game/Blueprints/Characters/BaseCharacterBP` OtherActor))
    (if (and (`|EnumInequality` (`/Game/Blueprints/Characters/BaseCharacterBP.Affiliation` _asbase_character_bp) (`self.Affiliation`)) (not (`KismetArrayLibrary.Array_Contains` (`self.HitCharacters`) _asbase_character_bp)))
      (`KismetArrayLibrary.Array_AddUnique` (`self.HitCharacters`) _asbase_character_bp)
      (bind (_returnvalue_x _returnvalue_y) (`KismetMathLibrary.BreakVector` (`KismetMathLibrary.GetDirectionUnitVector` (`self.K2_GetActorLocation`) (`self.K2_GetActorLocation` _asbase_character_bp))))
      (`self.LaunchCharacter` _asbase_character_bp (`KismetMathLibrary.MakeVector` (* (* _returnvalue_x 500.0) _action2knockback) (* (* _returnvalue_y 500.0) _action2knockback) (* 150.0 _action2knockback)) true true)
      (`self.ApplyDamage` _asbase_character_bp (`self.Action2Damage`)))))

(fn `UserConstructionScript`
  (`parent.UserConstructionScript`)
  (`SceneComponent.K2_AttachToComponent` (`self.WeaponPrimaryMesh`) (`self.Mesh`) "LeftHand" "KeepRelative" "KeepRelative" "KeepRelative" true)
  (`SceneComponent.K2_AttachToComponent` (`self.WeaponSecondaryMesh`) (`self.Mesh`) "RightHand" "KeepRelative" "KeepRelative" "KeepRelative" true)
  (`SceneComponent.K2_AttachToComponent` (`self.AttackCollision`) (`self.WeaponSecondaryMesh`) "RightHand" "KeepRelative" "KeepRelative" "KeepRelative" true))