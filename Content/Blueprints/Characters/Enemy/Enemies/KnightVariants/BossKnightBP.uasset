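; BossKnightBP is a boss variant of the knight enemy that displays an enlarged, custom-colored health bar.
; On BeginPlay it runs the parent logic, then casts its Widget component's widget to NPCHealth, sets its color from HealthColor and triples its render scale.
; Tick and construction only call the parent, and the overlap event is disabled, so the graphs add no other behavior.
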(event `self.ReceiveBeginPlay`
  (bind _returnvalue (`WidgetComponent.GetWidget` (`self.Widget`)))
  (`parent.ReceiveBeginPlay`)
  (set `/Game/Blueprints/Menus/Widgets/NPCHealth.Color` (`self.HealthColor`) (cast `/Game/Blueprints/Menus/Widgets/NPCHealth` _returnvalue :!pure true))
  (`Widget.SetRenderScale` _returnvalue (3.0 3.0)))

(event `self.ReceiveTick`
  (params (DeltaSeconds :type "Float (single-precision)"))
  (`parent.ReceiveTick` DeltaSeconds))

(fn `UserConstructionScript`
  (locals (NewLocalVar_0 :type "SlateColor Structure"))
  (`parent.UserConstructionScript`))