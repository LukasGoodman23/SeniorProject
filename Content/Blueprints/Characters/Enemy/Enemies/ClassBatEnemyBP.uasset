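; Bat enemy character Blueprint with a single melee ram attack, Action1.
; After a start delay, the attack enables the mesh-attached hitbox, then chains three timelines to move the mesh through wind-up, ram and return.
; Overlaps damage and launch opposing-affiliation characters away, once per attack via HitCharacters.
; The hitbox stays live until the return finishes; after an end delay, the action and hit list reset.
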(event `self.ReceiveBeginPlay`
  (`parent.ReceiveBeginPlay`))

(event `self.Action1`
  ;[0 0 0] Preparation
  (if (and (`self.Action1Ready`) (not (`self.PerformingAction`)))
    (set `self.PerformingAction` true)
    (set `self.Action1Ready` false)
    (`KismetSystemLibrary.RetriggerableDelay` (`self.Action1StartLag`))
    ;[0 0 0] Active Hitbox
    (set `self.SwordDamage` (`self.Action1Damage`))
    (set `self.KnockbackMultiplier` (`self.Action1Knockback`))
    (`PrimitiveComponent.SetCollisionEnabled` (`self.AttackCollision`) "QueryOnly")
    (bind (_direction _startlag) (`Timeline|StartLag` :!via `PlayFromStart`)
      (:`Update`
        (`SceneComponent.K2_SetRelativeTransform` (`self.Mesh`) (`KismetMathLibrary.TLerp` (`self.DefaultLocation`) (`self.WindUpLocation`) _startlag) false false))
      (:`Finished`
        (bind (_direction_2 _newtrack_0) (`Timeline|Attack` :!via `PlayFromStart`)
          (:`Update`
            (`SceneComponent.K2_SetRelativeTransform` (`self.Mesh`) (`KismetMathLibrary.TLerp` (`self.WindUpLocation`) (`self.RamLocation`) _newtrack_0) false false))
          (:`Finished`
            (bind (_direction_3 _newtrack_0_2) (`Timeline|EndLag` :!via `PlayFromStart`)
              (:`Update`
                (`SceneComponent.K2_SetRelativeTransform` (`self.Mesh`) (`KismetMathLibrary.TLerp` (`self.RamLocation`) (`self.DefaultLocation`) _newtrack_0_2) false false))
              (:`Finished`
                (`PrimitiveComponent.SetCollisionEnabled` (`self.AttackCollision`) "NoCollision")
                (`KismetSystemLibrary.RetriggerableDelay` (`self.Action1EndLag`))
                ;[0 0 0] End/Cleanup
                (set `self.PerformingAction` false)
                (`KismetArrayLibrary.Array_Clear` (`self.HitCharacters`))))))))))

(event `self.AttackCollision.OnComponentBeginOverlap`
  (params (OverlappedComponent :type "PrimitiveComponent Object Reference") (OtherActor :type "Actor Object Reference") (OtherComp :type "PrimitiveComponent Object Reference") (OtherBodyIndex :type Integer) (bFromSweep :type Boolean) (SweepResult :type "HitResult Structure (by ref)"))
  (bind _knockbackmultiplier (`self.KnockbackMultiplier`))
  ;[0 0 0] Melee Hit
  (if (!= OtherActor self)
    (bind _asbase_character_bp (cast `/Game/Blueprints/Characters/BaseCharacterBP` OtherActor))
    (if (and (`|EnumInequality` (`/Game/Blueprints/Characters/BaseCharacterBP.Affiliation` _asbase_character_bp) (`self.Affiliation`)) (not (`KismetArrayLibrary.Array_Contains` (`self.HitCharacters`) _asbase_character_bp)))
      (`KismetArrayLibrary.Array_AddUnique` (`self.HitCharacters`) _asbase_character_bp)
      (bind (_returnvalue_x _returnvalue_y) (`KismetMathLibrary.BreakVector` (`KismetMathLibrary.GetDirectionUnitVector` (`self.K2_GetActorLocation`) (`self.K2_GetActorLocation` _asbase_character_bp))))
      (`self.LaunchCharacter` _asbase_character_bp (`KismetMathLibrary.MakeVector` (* (* _returnvalue_x 500.0) _knockbackmultiplier) (* (* _returnvalue_y 500.0) _knockbackmultiplier) (* 150.0 _knockbackmultiplier)) true true)
      (`self.ApplyDamage` _asbase_character_bp (`self.SwordDamage`)))))

(fn `UserConstructionScript`
  (`parent.UserConstructionScript`)
  (`SceneComponent.K2_AttachToComponent` (`self.AttackCollision`) (`self.Mesh`) "None" "KeepRelative" "KeepRelative" "KeepRelative" true))