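; Training bat enemy Blueprint, a child enemy class that reacts to health changes.
; HealthChange prints the sum of current Health and the incoming delta, then calls CharacterBeaten when that sum is zero or below, without storing the new value here.
; BeginPlay only casts the player controller to PlayerControllerBP with nothing following, and construction defers to the parent.
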(event `self.ReceiveBeginPlay`
  (cast `/Game/Blueprints/PlayerControllerBP` (`GameplayStatics.GetPlayerController` 0)))

(event `self.ReceiveHealthChange`
  (params (HealthAdded :type Integer) (Attacker :type "Actor Object Reference"))
  (bind _returnvalue (+ HealthAdded (`self.Health`)))
  (`KismetSystemLibrary.PrintString` (`KismetStringLibrary.Conv_IntToString` _returnvalue))
  (if (<= _returnvalue 0)
    (`self.CharacterBeaten`)))

(fn `UserConstructionScript`
  (`parent.UserConstructionScript`))