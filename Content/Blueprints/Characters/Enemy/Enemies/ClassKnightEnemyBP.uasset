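; Knight enemy character with a light and a heavy sword attack.
; Each action plays its animation, then uses retriggerable delays to time start lag, an active hitbox window and end lag before restoring the animation blueprint.
; The sword hitbox damages and launches characters of other affiliations away from the knight, tracking victims so each is hit once per swing.
; Construction attaches the weapon and hitbox to the right hand.
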(event `self.Action1`
  ;[0 0 0] Preparation
  (if (and (`self.Action1Ready`) (not (`self.PerformingAction`)))
    (set `self.PerformingAction` true)
    (set `self.Action1Ready` false)
    (`SkeletalMeshComponent.PlayAnimation` (`self.Mesh`) "/Game/Characters/Heroes/anims/anim-knight/KnightAttkLight.KnightAttkLight" false)
    (`KismetSystemLibrary.RetriggerableDelay` (`self.Action1StartLag`))
    ;[0 0 0] Active Hitbox
    (set `self.SwordDamage` (`self.Action1Damage`))
    (set `self.KnockbackMultiplier` (`self.Action1Knockback`))
    (`PrimitiveComponent.SetCollisionEnabled` (`self.AttackCollision`) "QueryOnly")
    (`KismetSystemLibrary.RetriggerableDelay` (- (`self.Action1Duration`) (+ (`self.Action1StartLag`) (`self.Action1EndLag`))))
    (`PrimitiveComponent.SetCollisionEnabled` (`self.AttackCollision`) "NoCollision")
    (`KismetSystemLibrary.RetriggerableDelay` (`self.Action1EndLag`))
    ;[0 0 0] End/Cleanup
    (`SkeletalMeshComponent.SetAnimationMode` (`self.Mesh`) "AnimationBlueprint")
    (set `self.PerformingAction` false)
    (`KismetArrayLibrary.Array_Clear` (`self.HitCharacters`))))

(event `self.Action2`
  ;[0 0 0] Preparation
  (if (and (`self.Action2Ready`) (not (`self.PerformingAction`)))
    (set `self.PerformingAction` true)
    (set `self.Action2Ready` false)
    (`SkeletalMeshComponent.PlayAnimation` (`self.Mesh`) "/Game/Characters/Heroes/anims/anim-knight/KnightAttkHeavy.KnightAttkHeavy" false)
    (`KismetSystemLibrary.RetriggerableDelay` (`self.Action2StartLag`))
    ;[0 0 0] Active Hitbox
    (set `self.SwordDamage` (`self.Action2Damage`))
    (set `self.KnockbackMultiplier` (`self.Action2Knockback`))
    (`PrimitiveComponent.SetCollisionEnabled` (`self.AttackCollision`) "QueryOnly")
    (`KismetSystemLibrary.RetriggerableDelay` (- (`self.Action2Duration`) (+ (`self.Action2StartLag`) (`self.Action2EndLag`))))
    (`PrimitiveComponent.SetCollisionEnabled` (`self.AttackCollision`) "NoCollision")
    (`KismetSystemLibrary.RetriggerableDelay` (`self.Action2EndLag`))
    ;[0 0 0] End/Cleanup
    (`SkeletalMeshComponent.SetAnimationMode` (`self.Mesh`) "AnimationBlueprint")
    (set `self.PerformingAction` false)
    (`KismetArrayLibrary.Array_Clear` (`self.HitCharacters`))))

(event `self.AttackCollision.OnComponentBeginOverlap`
  (params (OverlappedComponent :type "PrimitiveComponent Object Reference") (OtherActor :type "Actor Object Reference") (OtherComp :type "PrimitiveComponent Object Reference") (OtherBodyIndex :type Integer) (bFromSweep :type Boolean) (SweepResult :type "HitResult Structure (by ref)"))
  (bind _knockbackmultiplier (`self.KnockbackMultiplier`))
  ;[0 0 0] Melee Hit
  (if (!= OtherActor self)
    (bind _asbase_character_bp (cast `/Game/Blueprints/Characters/BaseCharacterBP` OtherActor))
    (if (and (`|EnumInequality` (`/Game/Blueprints/Characters/BaseCharacterBP.Affiliation` _asbase_character_bp) (`self.Affiliation`)) (not (`KismetArrayLibrary.Array_Contains` (`self.HitCharacters`) _asbase_character_bp)))
      (`KismetArrayLibrary.Array_AddUnique` (`self.HitCharacters`) _asbase_character_bp)
      (bind (_returnvalue_x _returnvalue_y) (`KismetMathLibrary.BreakVector` (`KismetMathLibrary.GetDirectionUnitVector` (`self.K2_GetActorLocation`) (`self.K2_GetActorLocation` _asbase_character_bp))))
      (`self.LaunchCharacter` _asbase_character_bp (`KismetMathLibrary.MakeVector` (* (* _returnvalue_x 500.0) _knockbackmultiplier) (* (* _returnvalue_y 500.0) _knockbackmultiplier) (* 150.0 _knockbackmultiplier)) true true)
      (`self.ApplyDamage` _asbase_character_bp (`self.SwordDamage`)))))

(fn `UserConstructionScript`
  (`parent.UserConstructionScript`)
  (`SceneComponent.K2_AttachToComponent` (`self.WeaponPrimaryMesh`) (`self.Mesh`) "RightHand" "KeepRelative" "KeepRelative" "KeepRelative" true)
  (`SceneComponent.K2_AttachToComponent` (`self.AttackCollision`) (`self.WeaponPrimaryMesh`) "RightHand" "KeepRelative" "KeepRelative" "KeepRelative" true))