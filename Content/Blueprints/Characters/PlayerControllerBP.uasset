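; Player controller Blueprint that turns walk and camera-look axis inputs into movement and rotation of the possessed pawn.
; ResetControlledPawn caches the pawn reference and is called only on BeginPlay in this file.
; Walk axes add movement input along forward and right vectors built from control-rotation yaw alone, so camera pitch does not affect direction.
; Look axes feed the pawn's controller yaw and pitch input directly.
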(event `self.ReceiveBeginPlay`
  (`self.ResetControlledPawn`))

(event `InputAxis|WalkForward`
  (params (AxisValue :type "Float (single-precision)"))
  ;[0 0 0] Character movement
  (`Pawn.AddMovementInput` (`self.ControlledPawn`) (`KismetMathLibrary.GetForwardVector` (`KismetMathLibrary.MakeRotator` 0.0 0.0 (.yaw (`Pawn.GetControlRotation` (`self.ControlledPawn`))))) AxisValue false))

(event `InputAxis|CameraLookRight`
  (params (AxisValue :type "Float (single-precision)"))
  ;[0 0 0] Camera controls
  (`Pawn.AddControllerYawInput` (`self.ControlledPawn`) AxisValue))

(event `InputAxis|CameraLookUp`
  (params (AxisValue :type "Float (single-precision)"))
  ;[0 0 0] Camera controls
  (`Pawn.AddControllerPitchInput` (`self.ControlledPawn`) AxisValue))

(event `InputAxis|WalkRight`
  (params (AxisValue :type "Float (single-precision)"))
  ;[0 0 0] Character movement
  (`Pawn.AddMovementInput` (`self.ControlledPawn`) (`KismetMathLibrary.GetRightVector` (`KismetMathLibrary.MakeRotator` 0.0 0.0 (.yaw (`Pawn.GetControlRotation` (`self.ControlledPawn`))))) AxisValue false))

(fn `ResetControlledPawn`
  ;[0 0 0] Resets ControlledPawn when a new pawn is possessed
  (set `self.ControlledPawn` (`self.K2_GetPawn`)))

(fn `UserConstructionScript`)