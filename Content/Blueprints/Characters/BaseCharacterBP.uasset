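; Base character Blueprint providing shared health, damage, two action cooldowns and teammate-style revive interaction, with empty action, KnockOut and Revive hooks.
; Health changes clamp to valid bounds, call KnockOut at zero, and update the AI blackboard only for in-range results.
; Tick runs the cooldown timers, and the cached AI controller repossesses the character when a player controller leaves.
; Interact toggles manual reviving on a knocked-out character's KnockoutStatusBP component.
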(event `ReceiveHealthChange`
  (params (HealthAdded :type Integer))
  ;[0 0 0] Receive a change in Health (positive HealthAdded heals, negative Health Added damages)
  (if (not (`self.KnockedOut`))
    ;;[0 0 0] Prevent negative health (and handle KnockOut)
    (if (> (+ HealthAdded (`self.Health`)) 0)
      ;;[0 0 0] Prevent health greater than max
      (if (<= (+ HealthAdded (`self.Health`)) (`self.MaxHealth`))
        (bind _output_get (set `self.Health` (+ HealthAdded (`self.Health`))))
        (`BlackboardComponent.SetValueAsInt` (`AIController.Blackboard` (`self.AIControllerReference`)) "CurrentHealth" _output_get)
        (else
          (set `self.Health` (`self.MaxHealth`))))
      (else
        (set `self.Health` 0)
        (`self.KnockOut`)))))

(event `ApplyDamage`
  (params (TargetReceiver :type "/Game/Blueprints/Characters/BaseCharacterBP Object Reference") (DamageDealt :type Integer))
  ;[0 0 0] Apply damage to another BaseCharacterBP (TargetReceiver)
  ; DamageDealth should be positive and will be negated when applying damage
  (`self.ReceiveHealthChange` TargetReceiver (* DamageDealt -1)))

(event `self.ReceiveTick`
  (params (DeltaSeconds :type "Float (single-precision)"))
  ;[0 0 0] Cooldown handling
  (`|ExecutionSequence`
    (:`then_0`
      (if (not (`self.Action1Ready`))
        (bind _output_get (set `self.Action1CooldownTimer` (+ (`self.Action1CooldownTimer`) DeltaSeconds)))
        (if (>= _output_get (`self.Action1Cooldown`))
          (set `self.Action1CooldownTimer` 0.0)
          (set `self.Action1Ready` true))))
    (:`then_1`
      (if (not (`self.Action2Ready`))
        (bind _output_get_2 (set `self.Action2CooldownTimer` (+ (`self.Action2CooldownTimer`) DeltaSeconds)))
        (if (>= _output_get_2 (`self.Action2Cooldown`))
          (set `self.Action2CooldownTimer` 0.0)
          (set `self.Action2Ready` true))))))

(event `self.ReceiveBeginPlay`
  ;[0 0 0] AI Control
  (set `self.AIControllerReference` (`AIBlueprintHelperLibrary.GetAIController` self)))

(event `self.ReceiveUnpossessed`
  (params (OldController :type "Controller Object Reference"))
  ;[0 0 0] AI Control
  (if (`Controller.IsPlayerController` OldController)
    (`Controller.Possess` (`self.AIControllerReference`) self)))

(event `Action1`)

(event `Action2`)

(fn `Interact`
  (bind _output (`|GetArrayItem` (`self.InteractableCharacters`)))
  (if (not (`self.KnockedOut`))
    (`/Engine/EditorBlueprintResources/StandardMacros.IsValid` (`|GetArrayItem` (`self.InteractableCharacters`))
      (:`Is Valid`
        ;[0 0 0] Revive
        (if (`/Game/Blueprints/Characters/BaseCharacterBP.KnockedOut` _output)
          (set `self.InteractingWith` _output)
          (set `/Game/Blueprints/StatusComponents/StatusTypes/KnockoutStatusBP.ManualReviving` true (`self.GetComponentByClass` _output "/Game/Blueprints/StatusComponents/StatusTypes/KnockoutStatusBP.KnockoutStatusBP_C")))))))

(fn `KnockOut`)

(fn `Revive`)

(fn `StopInteracting`
  (bind _interactingwith (`self.InteractingWith`))
  (`/Engine/EditorBlueprintResources/StandardMacros.IsValid` (`self.InteractingWith`)
    (:`Is Valid`
      (`|ExecutionSequence`
        (:`then_0`
          ;[0 0 0] If reviving
          (if (`/Game/Blueprints/Characters/BaseCharacterBP.KnockedOut` _interactingwith)
            (set `/Game/Blueprints/StatusComponents/StatusTypes/KnockoutStatusBP.ManualReviving` false (`self.GetComponentByClass` _interactingwith "/Game/Blueprints/StatusComponents/StatusTypes/KnockoutStatusBP.KnockoutStatusBP_C"))))
        (:`then_1`
          (set `self.InteractingWith` null))))))

(fn `UserConstructionScript`
  (`PrimitiveComponent.SetSimulatePhysics` (`self.CapsuleComponent`) false)
  (`PrimitiveComponent.SetCollisionEnabled` (`self.AttackCollision`) "NoCollision")
  (set `self.Health` (`self.MaxHealth`)))